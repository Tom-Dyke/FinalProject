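; Scanner box actor that detects when a set of items has passed through it and flags the player's MousePawn as scanned.
; On overlap, it records each unique actor and prints the running count.
; Every Tick, it compares that count to NumberOfItems on SpawnItems actors attached to the controlled MousePawn.
; On a match, it sets Scanned on the pawn and clears the list.
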(event `self.ReceiveActorBeginOverlap`
  (params (OtherActor :type "Actor Object Reference"))
  (bind _actors_overlapped (`self.Actors Overlapped`))
  (if (== (`KismetArrayLibrary.Array_Find` (`self.Actors Overlapped`) OtherActor) -1)
    (`KismetArrayLibrary.Array_Add` _actors_overlapped OtherActor)
    (`KismetSystemLibrary.PrintString` (`KismetStringLibrary.Conv_IntToString` (`KismetArrayLibrary.Array_Length` _actors_overlapped)))))

(event `self.ReceiveTick`
  (params (DeltaSeconds :type "Float (single-precision)"))
  (bind _asmouse_pawn (cast `/Game/Blueprints/Actors/MousePawn` (`Controller.K2_GetPawn` (`GameplayStatics.GetPlayerController` 0))))
  (for _array_element (`self.GetAttachedActors` _asmouse_pawn true false)
    (bind _asspawn_items (cast `/Game/Blueprints/Actors/SpawnItems` _array_element))
    (if (== (`/Game/Blueprints/Actors/SpawnItems.Number of Items` _asspawn_items) (`KismetArrayLibrary.Array_Length` (`self.Actors Overlapped`)))
      (set `/Game/Blueprints/Actors/MousePawn.Scanned` true _asmouse_pawn)
      (`KismetArrayLibrary.Array_Clear` (`self.Actors Overlapped`)))))

(fn `UserConstructionScript`)