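; Rubbish spawner actor that drops a random-sized batch of physics-simulated, randomly scaled BinsRubbish actors at its own transform.
; BeginPlay registers it as the first-person character's SpawnBins and rolls the batch size once.
; Tick feeds a custom DoN Complete macro, whose Delay paces spawns about half a second apart until the count is reached.
; SpawnRubbish resets the macro to release another batch of the same size.
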(event `self.ReceiveBeginPlay`
  (bind _asbp_first_person_character (cast `/Game/FirstPerson/Blueprints/BP_FirstPersonCharacter` (`GameplayStatics.GetPlayerCharacter` 0)))
  (set `/Game/FirstPerson/Blueprints/BP_FirstPersonCharacter.SpawnBins` self _asbp_first_person_character)
  (set `self.Number of Boxes` (`KismetMathLibrary.RandomIntegerInRange` 4 12)))

(event `self.ReceiveTick`
  (params (DeltaSeconds :type "Float (single-precision)"))
  (`self.DoN Complete` (`self.Number of Boxes`) 0.5 :!label _label
    (:`Exit`
      (bind _returnvalue (`|SpawnActorFromClass` "/Game/Blueprints/Actors/BinsRubbish.BinsRubbish_C" (`self.GetTransform`) "Undefined" "OverrideRootScale" null null))
      (`self.SetActorScale3D` _returnvalue (`KismetMathLibrary.Conv_DoubleToVector` (`KismetMathLibrary.RandomFloatInRange` 0.5 0.8)))
      (bind _staticmesh (`/Game/Blueprints/Actors/BinsRubbish.StaticMesh` _returnvalue))
      (`PrimitiveComponent.SetSimulatePhysics` _staticmesh true)
      (set `PrimitiveComponent.CanCharacterStepUpOn` "ECB_No" _staticmesh))))

(event `Spawn Rubbish`
  (goto _label :!via `Reset`))

(fn `UserConstructionScript`)