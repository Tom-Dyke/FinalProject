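; Actor component that lets the player pick up its owning actor through an Interact event.
; Interact turns on physics for the owner's static mesh with physics-only collision, then teleports the owner to the first-person character's ItemConstraint with a yaw offset.
; The mesh is held by binding it to the character's capsule through that constraint rather than by attachment; the file contains no drop logic.
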(event `/Game/Blueprints/Interfaces/InteractInterface.Interact`
  (bind _returnvalue (`Actor.GetComponentByClass` (`self.GetOwner` self) "/Script/Engine.StaticMeshComponent"))
  (`self.Activate` false)
  (bind _output_get (set `self.Parent Static Mesh` _returnvalue))
  (`PrimitiveComponent.SetSimulatePhysics` _returnvalue true)
  (`PrimitiveComponent.SetSimulatePhysics` _output_get true)
  (`PrimitiveComponent.SetCollisionEnabled` (`self.Parent Static Mesh`) "PhysicsOnly")
  (bind _asbp_first_person_character (cast `/Game/FirstPerson/Blueprints/BP_FirstPersonCharacter` (`GameplayStatics.GetPlayerCharacter` 0)))
  (`Actor.K2_SetActorLocationAndRotation` (`self.GetOwner`) (.location (`SceneComponent.K2_GetComponentToWorld` (`/Game/FirstPerson/Blueprints/BP_FirstPersonCharacter.ItemConstraint` _asbp_first_person_character))) (`KismetMathLibrary.MakeRotator` (.roll (.rotation (`SceneComponent.K2_GetComponentToWorld` (`/Game/FirstPerson/Blueprints/BP_FirstPersonCharacter.ItemConstraint` _asbp_first_person_character)))) (.pitch (.rotation (`SceneComponent.K2_GetComponentToWorld` (`/Game/FirstPerson/Blueprints/BP_FirstPersonCharacter.ItemConstraint` _asbp_first_person_character)))) (- (.yaw (.rotation (`SceneComponent.K2_GetComponentToWorld` (`/Game/FirstPerson/Blueprints/BP_FirstPersonCharacter.ItemConstraint` _asbp_first_person_character)))) 90.0)) false true)
  (`PhysicsConstraintComponent.SetConstrainedComponents` (`/Game/FirstPerson/Blueprints/BP_FirstPersonCharacter.ItemConstraint` _asbp_first_person_character) (`self.Parent Static Mesh`) "None" (`Character.CapsuleComponent` _asbp_first_person_character) "None"))