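; Shelf component that lets the player restock an aisle shelf with the held box matching its AisleName.
; Interact on an empty shelf reveals the owner's attached actors, destroys the constrained held item and clears HeldObject; EmptyShelves hides those actors and sets ShelfEmpty.
; Wrong or already-stocked shelves show one-second popups, gated by resettable DoOnce nodes.
; Hovering hides the interact widget when nothing is held.
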(event `/Game/Blueprints/Interfaces/InteractInterface.Hovering`
  (params (InteractWidget :type "/Game/Blueprints/Widgets/InteractWidget Object Reference"))
  (if (== "None" (`/Game/FirstPerson/Blueprints/BP_FirstPersonCharacter.Held Object` (cast `/Game/FirstPerson/Blueprints/BP_FirstPersonCharacter` (`GameplayStatics.GetPlayerCharacter` 0) :!pure true)))
    (`Widget.SetVisibility` InteractWidget "Hidden")))

(event `/Game/Blueprints/Interfaces/InteractInterface.Interact`
  (bind _asbp_first_person_character (cast `/Game/FirstPerson/Blueprints/BP_FirstPersonCharacter` (`GameplayStatics.GetPlayerCharacter` 0) :!pure true))
  (if (== (`self.AisleName`) (`/Game/FirstPerson/Blueprints/BP_FirstPersonCharacter.Held Object` (cast `/Game/FirstPerson/Blueprints/BP_FirstPersonCharacter` (`GameplayStatics.GetPlayerCharacter` 0) :!pure true)))
    (if (`self.Shelf Empty`)
      (for _array_element (`Actor.GetAttachedActors` (`self.GetOwner`) true false)
        (`Actor.SetActorHiddenInGame` _array_element false))
      (bind _itemconstraint (`/Game/FirstPerson/Blueprints/BP_FirstPersonCharacter.ItemConstraint` _asbp_first_person_character)
        (:`then`
          (bind _outcomponent1 (`PhysicsConstraintComponent.GetConstrainedComponents` _itemconstraint))
          (`/Engine/EditorBlueprintResources/StandardMacros.IsValid` _outcomponent1
            (:`Is Valid`
              (`Actor.K2_DestroyActor` (`self.GetOwner` _outcomponent1))
              (`PhysicsConstraintComponent.BreakConstraint` _itemconstraint)
              (set `/Game/FirstPerson/Blueprints/BP_FirstPersonCharacter.Held Object` "None" _asbp_first_person_character))))
        (:`else`))
      (else
        (`self.NotEmpty`)))
    (else
      (`self.NotBox`))))

(event `Empty Shelves`
  (for _array_element (`Actor.GetAttachedActors` (`self.GetOwner`) true false)
    (`Actor.SetActorHiddenInGame` _array_element true)
    (set `self.Shelf Empty` true)))

(event `NotBox`
  (`/Engine/EditorBlueprintResources/StandardMacros.DoOnce` false :!label _label
    (:`Completed`
      (bind _pop_up (`self.Pop-Up`)
        (:`then`
          (`Widget.RemoveFromParent` _pop_up)
          (set `self.Pop-Up` null))
        (:`else`
          _))
      (bind _returnvalue (`|CreateWidget` "/Game/Blueprints/Widgets/Pop-UpWidget.Pop-UpWidget_C"))
      (bind _output_get (set `self.Pop-Up` _returnvalue))
      (set `/Game/Blueprints/Widgets/Pop-UpWidget.TextShown` "Wrong Shelf!" _output_get)
      (`UserWidget.AddToViewport` _output_get 0)
      (`KismetSystemLibrary.Delay` 1.0)
      (`Widget.RemoveFromParent` _output_get)
      (set `self.Pop-Up` null)
      (`self.Reset Widget`))))

(event `Reset Widget`
  (goto _label :!via `Reset`))

(event `NotEmpty`
  (`/Engine/EditorBlueprintResources/StandardMacros.DoOnce` false :!label _label_2
    (:`Completed`
      (bind _pop_up (`self.Pop-Up`)
        (:`then`
          (`Widget.RemoveFromParent` _pop_up)
          (set `self.Pop-Up` null))
        (:`else`
          _))
      (bind _returnvalue (`|CreateWidget` "/Game/Blueprints/Widgets/Pop-UpWidget.Pop-UpWidget_C"))
      (bind _output_get (set `self.Pop-Up` _returnvalue))
      (set `/Game/Blueprints/Widgets/Pop-UpWidget.TextShown` "Shelf already Stocked!" _output_get)
      (`UserWidget.AddToViewport` _output_get 0)
      (`KismetSystemLibrary.Delay` 1.0)
      (`Widget.RemoveFromParent` _output_get)
      (set `self.Pop-Up` null)
      (`self.ResetStocked`))))

(event `ResetStocked`
  (goto _label_2 :!via `Reset`))