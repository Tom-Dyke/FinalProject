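; BP_Base_play is a clickable play button actor for the LiminalMarket menu that loads the game level.
; Clicking its Box component starts a camera fade that holds when finished, waits briefly, then opens the "LM" level by name.
; BeginPlay only calls its parent, and Tick and overlap events are disabled.
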(event `self.ReceiveBeginPlay`
  (`parent.ReceiveBeginPlay`))

(event `self.Box.OnClicked`
  (params (TouchedComponent :type "PrimitiveComponent Object Reference") (ButtonPressed :type "Key Structure"))
  (`PlayerCameraManager.StartCameraFade` :`self` (`GameplayStatics.GetPlayerCameraManager` 0) :`ToAlpha` 1.0 :`bHoldWhenFinished` true)
  (`KismetSystemLibrary.Delay` 0.5)
  (`GameplayStatics.OpenLevel` "LM"))

(fn `UserConstructionScript`
  (`parent.UserConstructionScript`))