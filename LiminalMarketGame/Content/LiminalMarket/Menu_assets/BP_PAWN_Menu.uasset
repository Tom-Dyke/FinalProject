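; Menu pawn that moves its camera between placed viewpoints and lets the mouse operate widgets through a WidgetInteraction component.
; Each tick, the camera eases location and rotation toward the PositionArray actor selected by State, scaled by Speed and delta time.
; The interaction component follows the deprojected cursor ray.
; Left mouse press and release both call PressPointerKey, so the pointer key is never released here.
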(event `self.ReceiveTick`
  (params (DeltaSeconds :type "Float (single-precision)"))
  (bind _camera (`self.Camera`))
  (bind (_worldlocation _worlddirection) (`PlayerController.DeprojectMousePositionToWorld` (`GameplayStatics.GetPlayerController` 0)))
  (bind (_returnvalue_location _returnvalue_rotation) (`KismetMathLibrary.BreakTransform` (`SceneComponent.K2_GetComponentToWorld` _camera)))
  (bind _returnvalue (* DeltaSeconds (`self.Speed`)))
  (bind (_returnvalue_location_2 _returnvalue_rotation_2) (`KismetMathLibrary.BreakTransform` (`self.GetTransform` (`|GetArrayItem` (`self.PositionArray`) (`self.State`)))))
  (`SceneComponent.K2_SetWorldLocationAndRotation` _camera (`KismetMathLibrary.VLerp` _returnvalue_location _returnvalue_location_2 _returnvalue) (`KismetMathLibrary.RLerp` _returnvalue_rotation _returnvalue_rotation_2 _returnvalue) false false)
  (`SceneComponent.K2_SetWorldLocationAndRotation` (`self.WidgetInteraction`) _worldlocation (`KismetMathLibrary.Conv_VectorToRotator` _worlddirection) false false))

(event `Key|LeftMouseButton`
  (params (Key :type "Key Structure"))
  (bind _widgetinteraction (`self.WidgetInteraction`))
  (:`Pressed`
    (`WidgetInteractionComponent.PressPointerKey` _widgetinteraction "LeftMouseButton"))
  (:`Released`
    (`WidgetInteractionComponent.PressPointerKey` _widgetinteraction "LeftMouseButton")))

(fn `UserConstructionScript`)