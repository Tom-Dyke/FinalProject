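; BP_Base is a 3D text menu button, apparently a base Blueprint, that changes its look on mouse hover.
; A Box component's begin and end cursor-over events swap the Text3D front, back and bevel materials, while the extrude material is set to Textwhite both times.
; The material names read inverted: cursor entry applies Textplain and cursor exit applies Texthover.
; It has no click handling or construction logic.
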(event `self.Box.OnBeginCursorOver`
  (params (TouchedComponent :type "PrimitiveComponent Object Reference"))
  (bind _text3d (`self.Text3D`))
  (`Text3DComponent.SetExtrudeMaterial` _text3d "/Game/LiminalMarket/Menu_assets/BUttons/materials/textwhite.textwhite")
  (`Text3DComponent.SetBackMaterial` _text3d "/Game/LiminalMarket/Menu_assets/BUttons/materials/textplain.textplain")
  (`Text3DComponent.SetFrontMaterial` _text3d "/Game/LiminalMarket/Menu_assets/BUttons/materials/textplain.textplain")
  (`Text3DComponent.SetBevelMaterial` _text3d "/Game/LiminalMarket/Menu_assets/BUttons/materials/textplain.textplain"))

(event `self.Box.OnEndCursorOver`
  (params (TouchedComponent :type "PrimitiveComponent Object Reference"))
  (bind _text3d (`self.Text3D`))
  (`Text3DComponent.SetExtrudeMaterial` _text3d "/Game/LiminalMarket/Menu_assets/BUttons/materials/textwhite.textwhite")
  (`Text3DComponent.SetBackMaterial` _text3d "/Game/LiminalMarket/Menu_assets/BUttons/materials/texthover.texthover")
  (`Text3DComponent.SetFrontMaterial` _text3d "/Game/LiminalMarket/Menu_assets/BUttons/materials/texthover.texthover")
  (`Text3DComponent.SetBevelMaterial` _text3d "/Game/LiminalMarket/Menu_assets/BUttons/materials/texthover.texthover"))

(fn `UserConstructionScript`)