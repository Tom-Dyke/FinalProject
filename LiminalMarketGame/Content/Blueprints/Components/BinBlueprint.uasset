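; Interactable bin that disposes of the item the first-person player is holding when its held-object name matches the bin's name.
; On Interact, it finds the held item through the player's physics constraint and destroys that component's owning actor.
; It then breaks the constraint, clears the held-object name, reports a bin event to the player's game stats and calls TriggerThing with both flags off.
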(event `/Game/Blueprints/Interfaces/InteractInterface.Interact`
  (params (`Player Character` :type "/Game/FirstPerson/Blueprints/BP_FirstPersonCharacter Object Reference"))
  (bind _asbp_first_person_character (cast `/Game/FirstPerson/Blueprints/BP_FirstPersonCharacter` (`GameplayStatics.GetPlayerCharacter` 0) :!pure true))
  (bind _asbp_first_person_character_2 (cast `/Game/FirstPerson/Blueprints/BP_FirstPersonCharacter` (`GameplayStatics.GetPlayerCharacter` 0) :!pure true))
  (bind _itemconstraint (`/Game/FirstPerson/Blueprints/BP_FirstPersonCharacter.ItemConstraint` _asbp_first_person_character))
  (if (== (`self.BinName`) (`/Game/FirstPerson/Blueprints/BP_FirstPersonCharacter.Held Object` _asbp_first_person_character))
    (bind _outcomponent1 (`PhysicsConstraintComponent.GetConstrainedComponents` _itemconstraint))
    (`/Engine/EditorBlueprintResources/StandardMacros.IsValid` _outcomponent1
      (:`Is Valid`
        (`Actor.K2_DestroyActor` (`self.GetOwner` _outcomponent1))
        (`PhysicsConstraintComponent.BreakConstraint` _itemconstraint)
        (set `/Game/FirstPerson/Blueprints/BP_FirstPersonCharacter.Held Object` "None" _asbp_first_person_character_2)
        (`/Game/FirstPerson/Blueprints/BP_FirstPersonCharacter.Update Game Stats` _asbp_first_person_character_2 "Bin")
        (`/Game/FirstPerson/Blueprints/BP_FirstPersonCharacter.TriggerThing` _asbp_first_person_character_2 false false)))))