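; Actor component that makes its owning actor a note the player can pick up from day 4 and add to the clipboard.
; It hides the owner and disables its collision at start, then reveals it when the first-person character's NewDay event reports day 4.
; Interact updates the player's ClipboardWidget page limit and picked-up flag, shows a brief confirmation popup, then destroys the owner.
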(event `self.ReceiveBeginPlay`
  (bind _returnvalue (`self.GetOwner`))
  (bind _asbp_first_person_character (cast `/Game/FirstPerson/Blueprints/BP_FirstPersonCharacter` (`GameplayStatics.GetPlayerCharacter` 0)))
  (bind _output_get (set `self.First Person Character` _asbp_first_person_character))
  (add `/Game/FirstPerson/Blueprints/BP_FirstPersonCharacter.NewDay` _output_get (delegate `Day Change`))
  (`Actor.SetActorHiddenInGame` _returnvalue true)
  (`Actor.SetActorEnableCollision` _returnvalue false))

(event `Day Change`
  (params (`Day Number` :type Integer))
  (bind _returnvalue (`self.GetOwner`))
  (bind _output_get (set `self.Day Number` `Day Number`))
  (if (== _output_get 4)
    (`Actor.SetActorHiddenInGame` _returnvalue false)
    (`Actor.SetActorEnableCollision` _returnvalue true)))

(event `/Game/Blueprints/Interfaces/InteractInterface.Interact`
  (params (`Player Character` :type "/Game/FirstPerson/Blueprints/BP_FirstPersonCharacter Object Reference"))
  (bind _asclipboard_widget (cast `/Game/Blueprints/Widgets/ClipboardWidget` (`WidgetComponent.GetWidget` (`/Game/FirstPerson/Blueprints/BP_FirstPersonCharacter.Widget` `Player Character`))))
  (set `/Game/Blueprints/Widgets/ClipboardWidget.MaxWidgetIndex` 2 _asclipboard_widget)
  (set `/Game/Blueprints/Widgets/ClipboardWidget.PickedUp` true _asclipboard_widget)
  (`self.Pop-Up`
    (:`then`)
    (:`else`
      (bind _returnvalue (`|CreateWidget` "/Game/Blueprints/Widgets/Pop-UpWidget.Pop-UpWidget_C" null "Added to Clipboard"))
      (bind _output_get (set `self.Pop-Up` _returnvalue))
      (`UserWidget.AddToViewport` _output_get 0)
      (`KismetSystemLibrary.Delay` 1.0)
      (`Widget.RemoveFromParent` _output_get)
      (set `self.Pop-Up` null)
      (`Actor.K2_DestroyActor` (`self.GetOwner`)))))