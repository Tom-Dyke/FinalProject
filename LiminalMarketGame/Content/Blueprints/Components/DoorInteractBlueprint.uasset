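; DoorInteractBlueprint is a door interaction component that opens and closes its owner through the last ActorSequenceComponent found on BeginPlay.
; Interact flip-flops the sequence forward and reverse, or shows a one-second "Locked!" popup if DoorLocked, or if UseKeys is set and the player lacks ManagersKeys.
; InteractHold flip-flops DoorLocked when the player has ManagersKeys and UseKeys is off.
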(event `self.ReceiveBeginPlay`
  (bind _returnvalue (`Actor.K2_GetComponentsByClass` (`self.GetOwner` self) "/Script/ActorSequence.ActorSequenceComponent"))
  (if (`KismetArrayLibrary.Array_IsNotEmpty` _returnvalue)
    (for _array_element _returnvalue
      _)
    (set `self.ParentActorSequence` _array_element)))

(event `/Game/Blueprints/Interfaces/InteractInterface.Interact`
  (if (`self.Use Keys`)
    (bind _asbp_first_person_character (cast `/Game/FirstPerson/Blueprints/BP_FirstPersonCharacter` (`GameplayStatics.GetPlayerCharacter` 0)))
    (if (`/Game/FirstPerson/Blueprints/BP_FirstPersonCharacter.Managers Keys` _asbp_first_person_character)
      (if (`self.DoorLocked`) :!label _label
        (`self.Locked` :!label _label_2
          (:`then`)
          (:`else`
            (bind _returnvalue (`|CreateWidget` "/Game/Blueprints/Widgets/Pop-UpWidget.Pop-UpWidget_C"))
            (bind _output_get (set `self.Locked` _returnvalue))
            (set `/Game/Blueprints/Widgets/Pop-UpWidget.TextShown` "Locked!" _output_get)
            (`UserWidget.AddToViewport` _output_get 0)
            (`KismetSystemLibrary.Delay` 1.0)
            (`Widget.RemoveFromParent` _output_get)
            (set `self.Locked` null)))
        (else
          (`/Engine/EditorBlueprintResources/StandardMacros.FlipFlop`
            (:`A`
              (`ActorSequenceComponent.PlaySequence` (`self.ParentActorSequence`)))
            (:`B`
              (`MovieSceneSequencePlayer.PlayReverse` (`ActorSequenceComponent.SequencePlayer` (`self.ParentActorSequence`)))))))
      (else
        (goto _label_2)))
    (else
      (goto _label))))

(event `/Game/Blueprints/Interfaces/InteractInterface.InteractHold`
  (bind _asbp_first_person_character (cast `/Game/FirstPerson/Blueprints/BP_FirstPersonCharacter` (`GameplayStatics.GetPlayerCharacter` 0)))
  (if (and (`/Game/FirstPerson/Blueprints/BP_FirstPersonCharacter.Managers Keys` _asbp_first_person_character) (not (`self.Use Keys`)))
    (`/Engine/EditorBlueprintResources/StandardMacros.FlipFlop`
      (:`A`
        (set `self.DoorLocked` false))
      (:`B`
        (set `self.DoorLocked` true)))))