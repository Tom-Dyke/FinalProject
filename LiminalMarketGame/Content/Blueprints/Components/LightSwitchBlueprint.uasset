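; Light switch component that toggles the lights through the first-person player character when its Interact event fires.
; It casts player 0's character to BP_FirstPersonCharacter and reads its Lights flag to choose between LightsOff and LightsOn.
; Only the turn-on branch also rotates the owning actor, adding a fixed pitch offset to its current rotation with no matching reversal when switching off.
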(event `/Game/Blueprints/Interfaces/InteractInterface.Interact`
  (bind _returnvalue (`self.GetOwner`))
  (bind _asbp_first_person_character (cast `/Game/FirstPerson/Blueprints/BP_FirstPersonCharacter` (`GameplayStatics.GetPlayerCharacter` 0)))
  (if (`/Game/FirstPerson/Blueprints/BP_FirstPersonCharacter.Lights` _asbp_first_person_character)
    (`/Game/FirstPerson/Blueprints/BP_FirstPersonCharacter.Lights Off` _asbp_first_person_character false)
    (else
      (`/Game/FirstPerson/Blueprints/BP_FirstPersonCharacter.Lights On` _asbp_first_person_character)
      (`Actor.K2_SetActorRotation` _returnvalue (`KismetMathLibrary.MakeRotator` (.roll (`Actor.K2_GetActorRotation` _returnvalue)) (+ (.pitch (`Actor.K2_GetActorRotation` _returnvalue)) 100.0) (.yaw (`Actor.K2_GetActorRotation` _returnvalue))) false))))