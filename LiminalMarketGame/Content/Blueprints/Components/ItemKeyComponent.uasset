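; Actor component for the manager's keys item, which becomes visible and collidable once the player has finished their shift on day two.
; It binds to the player's new-day event to flag day two, then polls the shift state on Tick and reveals the owner's static mesh once.
; Interacting triggers the owner's dialogue message and sets the player's ManagersKeys flag.
; A separate Destry event destroys the owner after a short delay.
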(event `self.ReceiveBeginPlay`
  (bind _asbp_first_person_character (cast `/Game/FirstPerson/Blueprints/BP_FirstPersonCharacter` (`GameplayStatics.GetPlayerCharacter` 0)))
  (bind _output_get (set `self.Player Character` _asbp_first_person_character))
  (add `/Game/FirstPerson/Blueprints/BP_FirstPersonCharacter.NewDay` _output_get (delegate `Day`)))

(event `Day`
  (params (`Day Number` :type Integer))
  (switch `int` `Day Number`
    (:`2`
      (set `self.Day 2` true))))

(event `self.ReceiveTick`
  (params (DeltaSeconds :type "Float (single-precision)"))
  (bind _returnvalue (`Actor.GetComponentByClass` (`self.GetOwner`) "/Script/Engine.StaticMeshComponent"))
  (if (and (`self.Day 2`) (`/Game/FirstPerson/Blueprints/BP_FirstPersonCharacter.FinishedShift` (`self.Player Character`)))
    (`/Engine/EditorBlueprintResources/StandardMacros.DoOnce` false
      (:`Completed`
        (`SceneComponent.SetHiddenInGame` _returnvalue false false)
        (`PrimitiveComponent.SetCollisionEnabled` _returnvalue "QueryAndPhysics")))))

(event `/Game/Blueprints/Interfaces/InteractInterface.Interact`
  (params (`Player Character` :type "/Game/FirstPerson/Blueprints/BP_FirstPersonCharacter Object Reference"))
  (message `/Game/Blueprints/Interfaces/InteractInterface.Interact` (`Actor.GetComponentByClass` (`self.GetOwner`) "/Game/Blueprints/Components/DialogueComponent.DialogueComponent_C") `Player Character`)
  (set `/Game/FirstPerson/Blueprints/BP_FirstPersonCharacter.Managers Keys` true (`self.Player Character`)))

(event `Destry`
  (`KismetSystemLibrary.Delay` 0.5)
  (`Actor.K2_DestroyActor` (`self.GetOwner`)))