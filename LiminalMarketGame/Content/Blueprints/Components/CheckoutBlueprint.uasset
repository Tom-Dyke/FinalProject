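; Checkout component that lets the player take over a register camera to serve a waiting customer.
; On Interact with the lights on, it finds an attached actor with a camera component and, if a customer waits, triggers the player's checkout camera and possesses that actor as a MousePawn.
; With the lights off, it briefly shows a popup saying to turn on the power, using a resettable DoOnce to block repeats.
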(event `/Game/Blueprints/Interfaces/InteractInterface.Interact`
  (params (`Player Character` :type "/Game/FirstPerson/Blueprints/BP_FirstPersonCharacter Object Reference"))
  (bind _output_get (set `self.Player Character` `Player Character`))
  (if (`/Game/FirstPerson/Blueprints/BP_FirstPersonCharacter.Lights` _output_get)
    (for _array_element (`Actor.GetAttachedActors` (`self.GetOwner`) true false)
      (if (`KismetArrayLibrary.Array_IsNotEmpty` (`Actor.K2_GetComponentsByClass` _array_element "/Script/Engine.CameraComponent"))
        (set `self.Camera Actor Reference` _array_element)
        (if (`/Game/FirstPerson/Blueprints/BP_FirstPersonCharacter.CustomerWaiting` (`self.Player Character`))
          (`/Game/FirstPerson/Blueprints/BP_FirstPersonCharacter.CheckoutCamera` (`self.Player Character`))
          (bind _asmouse_pawn (cast `/Game/Blueprints/Actors/MousePawn` (`self.Camera Actor Reference`)))
          (`/Game/Blueprints/Actors/MousePawn.On Possess` _asmouse_pawn (`self.Player Character`))
          (`Controller.Possess` (`GameplayStatics.GetPlayerController` 0) _asmouse_pawn))))
    (else
      (`/Engine/EditorBlueprintResources/StandardMacros.DoOnce` false :!label _label
        (:`Completed`
          (bind _pop_up (`self.Pop-Up`)
            (:`then`
              (`Widget.RemoveFromParent` _pop_up)
              (set `self.Pop-Up` null))
            (:`else`
              _))
          (bind _returnvalue (`|CreateWidget` "/Game/Blueprints/Widgets/Pop-UpWidget.Pop-UpWidget_C" null "Click to Interact"))
          (bind _output_get_2 (set `self.Pop-Up` _returnvalue))
          (set `/Game/Blueprints/Widgets/Pop-UpWidget.TextShown` "You must turn on the power!" _output_get_2)
          (`UserWidget.AddToViewport` _output_get_2 0)
          (`KismetSystemLibrary.Delay` 1.0)
          (`Widget.RemoveFromParent` _output_get_2)
          (set `self.Pop-Up` null)
          (`self.Reset Widget`))))))

(event `Reset Widget`
  (goto _label :!via `Reset`))