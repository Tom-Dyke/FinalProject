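; Actor component that lets a player character pick up and carry its owning actor as a physics object.
; Interact and Pick-Up both call the player's BreakOld, activate the component, then set the owner's static mesh to simulate physics with physics-only collision.
; The owner teleports to the player's ItemConstraint with a yaw offset, and that constraint then binds the mesh to the player's capsule.
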(event `/Game/Blueprints/Interfaces/InteractInterface.Interact`
  (params (`Player Character` :type "/Game/FirstPerson/Blueprints/BP_FirstPersonCharacter Object Reference"))
  (bind _player_character (`self.Player Character`))
  (bind _returnvalue (`Actor.GetComponentByClass` (`self.GetOwner` self) "/Script/Engine.StaticMeshComponent"))
  (bind _output_get (set `self.Player Character` `Player Character`))
  (`/Game/FirstPerson/Blueprints/BP_FirstPersonCharacter.BreakOld` _output_get)
  (`self.Activate` false :!label _label)
  (bind _output_get_2 (set `self.Parent Static Mesh` _returnvalue))
  (`PrimitiveComponent.SetSimulatePhysics` _returnvalue true)
  (`PrimitiveComponent.SetSimulatePhysics` _output_get_2 true)
  (`PrimitiveComponent.SetCollisionEnabled` (`self.Parent Static Mesh`) "PhysicsOnly")
  (`Actor.K2_SetActorLocationAndRotation` (`self.GetOwner`) (.location (`SceneComponent.K2_GetComponentToWorld` (`/Game/FirstPerson/Blueprints/BP_FirstPersonCharacter.ItemConstraint` (`self.Player Character`)))) (`KismetMathLibrary.MakeRotator` (.roll (.rotation (`SceneComponent.K2_GetComponentToWorld` (`/Game/FirstPerson/Blueprints/BP_FirstPersonCharacter.ItemConstraint` (`self.Player Character`))))) (.pitch (.rotation (`SceneComponent.K2_GetComponentToWorld` (`/Game/FirstPerson/Blueprints/BP_FirstPersonCharacter.ItemConstraint` (`self.Player Character`))))) (- (.yaw (.rotation (`SceneComponent.K2_GetComponentToWorld` (`/Game/FirstPerson/Blueprints/BP_FirstPersonCharacter.ItemConstraint` (`self.Player Character`))))) 90.0)) false true)
  (`PhysicsConstraintComponent.SetConstrainedComponents` (`/Game/FirstPerson/Blueprints/BP_FirstPersonCharacter.ItemConstraint` _player_character) (`self.Parent Static Mesh`) "None" (`Character.CapsuleComponent` _player_character) "None"))

(event `Pick-Up`
  (params (`Player Character` :type "/Game/FirstPerson/Blueprints/BP_FirstPersonCharacter Object Reference"))
  (bind _output_get (set `self.Player Character` `Player Character`))
  (`/Game/FirstPerson/Blueprints/BP_FirstPersonCharacter.BreakOld` _output_get)
  (goto _label))