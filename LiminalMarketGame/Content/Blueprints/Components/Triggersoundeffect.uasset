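; Actor component for a TriggerBox that plays a one-shot positional sound on a specific in-game day.
; On BeginPlay it caches the first-person player character and binds to the owning box's begin-overlap event.
; The first overlap by any actor passes a DoOnce, then spawns the attenuated sound at a set location if the player's DayNumber matches.
; A first overlap on another day still consumes the trigger.
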(event `self.ReceiveBeginPlay`
  (bind _asbp_first_person_character (cast `/Game/FirstPerson/Blueprints/BP_FirstPersonCharacter` (`GameplayStatics.GetPlayerCharacter` 0)))
  (set `self.As BP First Person Character` _asbp_first_person_character)
  (bind _astrigger_box (cast `TriggerBox` (`self.GetOwner`)))
  (add `Actor.OnActorBeginOverlap` _astrigger_box (delegate `Onoverlap`)))

(event `Onoverlap`
  (params (OverlappedActor :type "Actor Object Reference") (OtherActor :type "Actor Object Reference"))
  (`/Engine/EditorBlueprintResources/StandardMacros.DoOnce` false
    (:`Completed`
      (if (== (`/Game/FirstPerson/Blueprints/BP_FirstPersonCharacter.DayNumber` (`self.As BP First Person Character`)) (`self.Daynumber`))
        (bind _returnvalue (`GameplayStatics.SpawnSoundAtLocation` (`self.Sound`) (`self.Location`) (struct) 1.0 1.0 0.0 (`self.Attenuation Settings`) null))
        (`AudioComponent.Play` _returnvalue 0.0)))))