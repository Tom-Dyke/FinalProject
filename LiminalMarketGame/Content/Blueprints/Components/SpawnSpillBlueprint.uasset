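; Actor component that turns its owner into a spill that can appear, have a janitor spawned at it, and be reset.
; On BeginPlay it registers itself in the first-person character's SpillSpawner array.
; SpawnSpill reveals the owner's decal and mesh and enables box collision, gated by a DoOnce, while SpawnJanitor spawns a JanitorSpills actor at the owner's transform.
; ResetSpill re-arms the gate, hides the spill, disables collision and destroys the janitor.
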(event `self.ReceiveBeginPlay`
  (bind _asbp_first_person_character (cast `/Game/FirstPerson/Blueprints/BP_FirstPersonCharacter` (`GameplayStatics.GetPlayerCharacter` 0)))
  (`KismetArrayLibrary.Array_AddUnique` (`/Game/FirstPerson/Blueprints/BP_FirstPersonCharacter.SpillSpawner` _asbp_first_person_character) self))

(event `Spawn Spill`
  (bind _returnvalue (`self.GetOwner`))
  (`/Engine/EditorBlueprintResources/StandardMacros.DoOnce` false :!label _label
    (:`Completed`
      (`SceneComponent.SetHiddenInGame` (`Actor.GetComponentByClass` _returnvalue "/Script/Engine.DecalComponent") false false)
      (`SceneComponent.SetHiddenInGame` (`Actor.GetComponentByClass` _returnvalue "/Script/Engine.StaticMeshComponent") false false)
      (`PrimitiveComponent.SetCollisionEnabled` (`Actor.GetComponentByClass` _returnvalue "/Script/Engine.BoxComponent") "QueryAndPhysics")
      (set `self.Spill` true))))

(event `SpawnJanitor`
  (bind _returnvalue (`|SpawnActorFromClass` "/Game/Blueprints/Actors/JanitorSpills.JanitorSpills_C" (`Actor.GetTransform` (`self.GetOwner`)) "Undefined" "OverrideRootScale" null null))
  (set `self.Janitor` _returnvalue))

(event `Reset Spill`
  (bind _returnvalue (`self.GetOwner`))
  (`|ExecutionSequence`
    (:`then_0`
      (goto _label :!via `Reset`))
    (:`then_1`
      (`SceneComponent.SetHiddenInGame` (`Actor.GetComponentByClass` _returnvalue "/Script/Engine.DecalComponent") true false)
      (`SceneComponent.SetHiddenInGame` (`Actor.GetComponentByClass` _returnvalue "/Script/Engine.StaticMeshComponent") true false)
      (`PrimitiveComponent.SetCollisionEnabled` (`Actor.GetComponentByClass` _returnvalue "/Script/Engine.BoxComponent") "NoCollision")
      (`Actor.K2_DestroyActor` (`self.Janitor`))
      (set `self.Spill` false))))