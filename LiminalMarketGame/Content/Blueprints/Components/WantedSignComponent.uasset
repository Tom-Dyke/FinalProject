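; Actor component for an interactable wanted sign that stages an intro dialogue with a Manager.
; It registers itself on the first-person character and destroys its owner when that character's new-day event fires.
; Interact briefly disables input, unhides the attached Manager, teleports and turns the player, then triggers the Manager's DialogueComponent.
; DeleteIntro removes both Manager and sign after a short delay.
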(event `self.ReceiveBeginPlay`
  (bind _asbp_first_person_character (cast `/Game/FirstPerson/Blueprints/BP_FirstPersonCharacter` (`GameplayStatics.GetPlayerCharacter` 0)))
  (set `/Game/FirstPerson/Blueprints/BP_FirstPersonCharacter.WantedSign` self _asbp_first_person_character)
  (add `/Game/FirstPerson/Blueprints/BP_FirstPersonCharacter.NewDay` _asbp_first_person_character (delegate `Day`)))

(event `DeleteIntro`
  (`KismetSystemLibrary.Delay` 1.0)
  (`Actor.K2_DestroyActor` (`self.Manager`))
  (`Actor.K2_DestroyActor` (`self.GetOwner`)))

(event `Day`
  (params (`Day Number` :type Integer))
  (switch `int` `Day Number`
    (:`Default`
      (`Actor.K2_DestroyActor` (`self.GetOwner`)))))

(event `/Game/Blueprints/Interfaces/InteractInterface.Interact`
  (params (`Player Character` :type "/Game/FirstPerson/Blueprints/BP_FirstPersonCharacter Object Reference"))
  (bind _returnvalue (`self.GetOwner`))
  (bind _output_get (set `self.Player Character` `Player Character`))
  (`Actor.DisableInput` _output_get (`GameplayStatics.GetPlayerController` 0))
  (`KismetSystemLibrary.Delay` 1.0)
  (for _array_element (`Actor.GetAttachedActors` _returnvalue true false)
    (set `self.Manager` _array_element))
  (`Actor.SetActorHiddenInGame` _array_element false)
  (`Controller.SetControlRotation` (`GameplayStatics.GetPlayerController` 0) (`KismetMathLibrary.MakeRotator` 0.0 0.0 270.0))
  (`Actor.K2_TeleportTo` :`self` (`self.Player Character`) :`DestLocation` (- (`Actor.K2_GetActorLocation` _returnvalue) (139.0 0.0 90.0)))
  (`KismetSystemLibrary.Delay` 0.1)
  (`Actor.EnableInput` (`self.Player Character`) (`GameplayStatics.GetPlayerController` 0))
  (message `/Game/Blueprints/Interfaces/InteractInterface.Interact` (`Actor.GetComponentByClass` (`self.Manager`) "/Game/Blueprints/Components/DialogueComponent.DialogueComponent_C") (`self.Player Character`)))