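; Actor component that runs player dialogue by using a behavior tree as the conversation logic.
; A dedicated DialogueAIController spawns at BeginPlay to host the tree.
; Interact checks out the player's camera, disables movement, shows the dialogue widget with UI-only input, then runs the tree and passes the widget through the blackboard.
; The widget's exit callback stops the tree, removes the widget, and restores game input and walking.
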(event `self.ReceiveBeginPlay`
  (bind _returnvalue (`|SpawnActorFromClass` "/Game/Blueprints/AI/Dialogue/DialogueAIController.DialogueAIController_C" (`Actor.GetTransform` (`self.GetOwner`)) "Undefined" "OverrideRootScale" null null))
  (set `self.AI Controller` _returnvalue))

(event `/Game/Blueprints/Interfaces/InteractInterface.Interact`
  (params (`Player Character` :type "/Game/FirstPerson/Blueprints/BP_FirstPersonCharacter Object Reference"))
  (bind _asplayer_controller (cast `PlayerController` (`Pawn.GetController` `Player Character`) :!pure true))
  (bind _output_get (set `self.Player Character` `Player Character`))
  (`/Game/FirstPerson/Blueprints/BP_FirstPersonCharacter.CheckoutCamera` _output_get)
  (`CharacterMovementComponent.DisableMovement` (`Character.CharacterMovement` `Player Character`))
  (bind _returnvalue (`|CreateWidget` "/Game/Blueprints/Widgets/DialogueWidget.DialogueWidget_C" _asplayer_controller))
  (bind _output_get_2 (set `self.Dialogue Widget` _returnvalue))
  (add `/Game/Blueprints/Widgets/DialogueWidget.OnExit` _output_get_2 (delegate `OnExit_Event`))
  (`UserWidget.AddToViewport` _output_get_2 0)
  (`WidgetBlueprintLibrary.SetInputMode_UIOnlyEx` _asplayer_controller _output_get_2)
  (set `PlayerController.bShowMouseCursor` true _asplayer_controller)
  (`AIController.RunBehaviorTree` (`self.AI Controller`) (`self.Dialogue Tree`))
  (bind _blackboardcomponent (`AIController.UseBlackboard` (`self.AI Controller`) "/Game/Blueprints/AI/Dialogue/DialogueBlackboard.DialogueBlackboard"))
  (`BlackboardComponent.SetValueAsObject` _blackboardcomponent "DialogueWidget" (`self.Dialogue Widget`)))

(event `OnExit_Event`
  (bind _asplayer_controller (cast `PlayerController` (`Pawn.GetController` (stale `/Game/Blueprints/Interfaces/InteractInterface.Interact` `Player Character`)) :!pure true))
  (`WidgetBlueprintLibrary.SetInputMode_GameOnly` _asplayer_controller)
  (set `PlayerController.bShowMouseCursor` false _asplayer_controller)
  (`BrainComponent.StopLogic` (`AIController.BrainComponent` (`self.AI Controller`)) "exit")
  (`Widget.RemoveFromParent` (`self.Dialogue Widget`))
  (`CharacterMovementComponent.SetMovementMode` (`Character.CharacterMovement` (`self.Player Character`)) "MOVE_Walking" 0))