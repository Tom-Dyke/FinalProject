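; Actor component for the clock-in machine, letting the player clock in and, once the shift is finished, clock out.
; It registers its owner with the first-person character and binds to the new-day event, hiding the machine and its attachments on day 0.
; Interaction alternates through paired DoOnce gates, updating the character and clipboard checkbox.
; It swaps machine meshes by matching attached actors' display names, also disabling a blocking volume's collision on clock-in.
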(event `self.ReceiveBeginPlay`
  (bind _returnvalue (`self.GetOwner`))
  (bind _asbp_first_person_character (cast `/Game/FirstPerson/Blueprints/BP_FirstPersonCharacter` (`GameplayStatics.GetPlayerCharacter` 0)))
  (set `/Game/FirstPerson/Blueprints/BP_FirstPersonCharacter.ClockInMachine Ref` (`self.GetOwner`) _asbp_first_person_character)
  (add `/Game/FirstPerson/Blueprints/BP_FirstPersonCharacter.NewDay` _asbp_first_person_character (delegate `Day`))
  (bind _output_get (set `self.Out Actors` (`Actor.GetAttachedActors` _returnvalue true false)))
  (`KismetArrayLibrary.Array_Add` _output_get _returnvalue))

(event `Day`
  (params (`Day Number` :type Integer))
  (switch `int` `Day Number`
    (:`Default`
      (for _array_element (`self.Out Actors`)
        (`Actor.SetActorHiddenInGame` _array_element false)
        (`Actor.SetActorEnableCollision` _array_element true)))
    (:`0`
      (for _array_element_2 (`self.Out Actors`)
        (`Actor.SetActorHiddenInGame` _array_element_2 true)
        (`Actor.SetActorEnableCollision` _array_element_2 false)))))

(event `/Game/Blueprints/Interfaces/InteractInterface.Interact`
  (params (`Player Character` :type "/Game/FirstPerson/Blueprints/BP_FirstPersonCharacter Object Reference"))
  (bind _player_character (`self.Player Character`))
  (bind _player_character_2 (`self.Player Character`))
  (bind _output_get (set `self.Player Character` `Player Character`))
  (if (`/Game/FirstPerson/Blueprints/BP_FirstPersonCharacter.ClockedIn` _output_get)
    (`/Engine/EditorBlueprintResources/StandardMacros.DoOnce` false :!label _label
      (:`Completed`
        (if (`/Game/FirstPerson/Blueprints/BP_FirstPersonCharacter.FinishedShift` _output_get)
          (set `/Game/FirstPerson/Blueprints/BP_FirstPersonCharacter.ClockedIn` false _player_character)
          (`/Game/FirstPerson/Blueprints/BP_FirstPersonCharacter.Clock-Out` _player_character)
          (`self.Clock Out`)
          (for _array_element (`Actor.GetAttachedActors` (`self.GetOwner`) true false)
            (if (`KismetStringLibrary.EqualEqual_StrStr` (`KismetSystemLibrary.GetDisplayName` _array_element) "clocking_mahionce3")
              (`Actor.SetActorHiddenInGame` _array_element true)
              (elif (`KismetStringLibrary.EqualEqual_StrStr` (`KismetSystemLibrary.GetDisplayName` _array_element) "clocking_mahionce2")
                (`Actor.SetActorHiddenInGame` _array_element false))))
          (goto _label_2 :!via `Reset`))))
    (else
      (`/Engine/EditorBlueprintResources/StandardMacros.DoOnce` false :!label _label_2
        (:`Completed`
          (set `/Game/FirstPerson/Blueprints/BP_FirstPersonCharacter.ClockedIn` true _player_character_2)
          (`/Game/FirstPerson/Blueprints/BP_FirstPersonCharacter.Clock-In` _player_character_2)
          (`self.Clock In`)
          (for _array_element_2 (`Actor.GetAttachedActors` (`self.GetOwner`) true false)
            (if (`KismetStringLibrary.EqualEqual_StrStr` (`KismetSystemLibrary.GetDisplayName` _array_element_2) "clocking_mahionce2")
              (`Actor.SetActorHiddenInGame` _array_element_2 true)
              (elif (`KismetStringLibrary.EqualEqual_StrStr` (`KismetSystemLibrary.GetDisplayName` _array_element_2) "clocking_mahionce3")
                (`Actor.SetActorHiddenInGame` _array_element_2 false)
                (elif (`KismetStringLibrary.EqualEqual_StrStr` (`KismetSystemLibrary.GetDisplayName` _array_element_2) "BlockingVolume7")
                  (`Actor.SetActorEnableCollision` _array_element_2 false)))))
          (goto _label :!via `Reset`))))))

(event `Clock In`
  (bind _asclipboard_widget (cast `/Game/Blueprints/Widgets/ClipboardWidget` (`WidgetComponent.GetWidget` (`/Game/FirstPerson/Blueprints/BP_FirstPersonCharacter.Widget` (`self.Player Character`)))))
  (`CheckBox.SetIsChecked` (`/Game/Blueprints/Widgets/ClipboardWidget.ClockIn` _asclipboard_widget) true))

(event `Clock Out`
  (bind _asclipboard_widget (cast `/Game/Blueprints/Widgets/ClipboardWidget` (`WidgetComponent.GetWidget` (`/Game/FirstPerson/Blueprints/BP_FirstPersonCharacter.Widget` (`self.Player Character`)))))
  (`CheckBox.SetIsChecked` (`/Game/Blueprints/Widgets/ClipboardWidget.ClockIn` _asclipboard_widget) false))