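; Box spawner actor that drops a set number of physics-enabled delivery boxes at its transform, then empties matching store shelves.
; Tick drives a custom DoN Complete macro that spaces spawns by a half-second delay and fires Finished once at the limit.
; On finish, each box's chosen name is matched against ShelfBlueprint aisle names on static mesh actors, consuming one name per emptied shelf.
; The SpawnBoxes event resets the macro for another delivery.
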(event `self.ReceiveTick`
  (params (DeltaSeconds :type "Float (single-precision)"))
  (bind _returnvalue (`KismetArrayLibrary.Array_Find` (`self.Spawned Boxes Names`) (`/Game/Blueprints/Components/ShelfBlueprint.AisleName` (`self.Shelf Blueprint Reference`))))
  (`self.DoN Complete` (`self.Number of Boxes`) 0.5 :!label _label
    (:`Exit`
      (bind _returnvalue_2 (`|SpawnActorFromClass` "/Game/Blueprints/Components/DeliveryBoxes.DeliveryBoxes_C" (`self.GetTransform`) "Undefined" "OverrideRootScale" null null))
      (bind _staticmesh (`/Game/Blueprints/Components/DeliveryBoxes.StaticMesh` _returnvalue_2))
      (`PrimitiveComponent.SetSimulatePhysics` _staticmesh true)
      (set `PrimitiveComponent.CanCharacterStepUpOn` "ECB_No" _staticmesh)
      (`KismetArrayLibrary.Array_Add` (`self.Spawned Boxes`) _returnvalue_2))
    (:`Finished`
      (for _array_element (`self.Spawned Boxes`)
        (`KismetArrayLibrary.Array_Add` (`self.Spawned Boxes Names`) (`/Game/Blueprints/Components/DeliveryBoxes.ChosenBox` _array_element)))
      (`KismetArrayLibrary.Array_Clear` (`self.Spawned Boxes`))
      (bind _outactors (`GameplayStatics.GetAllActorsOfClass` "/Script/Engine.StaticMeshActor"))
      (for _array_element_2 _outactors
        (bind _returnvalue_3 (`self.GetComponentByClass` _array_element_2 "/Game/Blueprints/Components/ShelfBlueprint.ShelfBlueprint_C"))
        (if (`KismetSystemLibrary.IsValid` _returnvalue_3)
          (set `self.Shelf Blueprint Reference` _returnvalue_3)
          (if (!= _returnvalue -1)
            (`KismetArrayLibrary.Array_Remove` (`self.Spawned Boxes Names`) _returnvalue)
            (`/Game/Blueprints/Components/ShelfBlueprint.Empty Shelves` (`self.Shelf Blueprint Reference`))))))))

(event `Spawn Boxes`
  (goto _label :!via `Reset`))

(fn `UserConstructionScript`)