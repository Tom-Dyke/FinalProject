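; An actor component for the clock-in machine that makes it present only on day 0.
; On BeginPlay it registers its owner as the first-person character's clock-in machine, binds to that character's new-day event, and caches the owner with its directly attached actors.
; The day handler shows those actors with collision on day 0 and hides them without collision on any other day.
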(event `self.ReceiveBeginPlay`
  (bind _returnvalue (`self.GetOwner`))
  (bind _asbp_first_person_character (cast `/Game/FirstPerson/Blueprints/BP_FirstPersonCharacter` (`GameplayStatics.GetPlayerCharacter` 0)))
  (set `/Game/FirstPerson/Blueprints/BP_FirstPersonCharacter.ClockInMachine Ref` (`self.GetOwner`) _asbp_first_person_character)
  (add `/Game/FirstPerson/Blueprints/BP_FirstPersonCharacter.NewDay` _asbp_first_person_character (delegate `Day`))
  (bind _output_get (set `self.Out Actors` (`Actor.GetAttachedActors` _returnvalue true false)))
  (`KismetArrayLibrary.Array_Add` _output_get _returnvalue))

(event `Day`
  (params (`Day Number` :type Integer))
  (switch `int` `Day Number`
    (:`Default`
      (for _array_element (`self.Out Actors`)
        (`Actor.SetActorHiddenInGame` _array_element true)
        (`Actor.SetActorEnableCollision` _array_element false)
        (if (`KismetStringLibrary.EqualEqual_StrStr` (`KismetSystemLibrary.GetDisplayName` _array_element) "clocking_mahionce4")
          (`Actor.SetActorHiddenInGame` _array_element true))))
    (:`0`
      (for _array_element_2 (`self.Out Actors`)
        (`Actor.SetActorHiddenInGame` _array_element_2 false)
        (`Actor.SetActorEnableCollision` _array_element_2 true)))))