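; Actor component that spawns a physics-simulated BinsRubbish item just above its owning actor.
; On BeginPlay it adds itself to the first-person character's SpawnRubbishComponent list.
; A DoOnce on Tick spawns a single half-scale rubbish item that characters cannot step up on.
; The SpawnRubbish event resets that gate, so the next tick spawns another.
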(event `self.ReceiveBeginPlay`
  (bind _asbp_first_person_character (cast `/Game/FirstPerson/Blueprints/BP_FirstPersonCharacter` (`GameplayStatics.GetPlayerCharacter` 0)))
  (`KismetArrayLibrary.Array_AddUnique` (`/Game/FirstPerson/Blueprints/BP_FirstPersonCharacter.SpawnRubbishComponent` _asbp_first_person_character) self))

(event `self.ReceiveTick`
  (params (DeltaSeconds :type "Float (single-precision)"))
  (`/Engine/EditorBlueprintResources/StandardMacros.DoOnce` false :!label _label
    (:`Completed`
      (bind _returnvalue (`|SpawnActorFromClass` "/Game/Blueprints/Actors/BinsRubbish.BinsRubbish_C" (`KismetMathLibrary.MakeTransform` (+ (.location (`Actor.GetTransform` (`self.GetOwner`))) (0.0 0.0 60.0)) (.rotation (`Actor.GetTransform` (`self.GetOwner`))) (.scale (`Actor.GetTransform` (`self.GetOwner`)))) "Undefined" "OverrideRootScale" null null))
      (bind _output_get (set `self.SpawnedRubbish` _returnvalue))
      (`Actor.SetActorScale3D` _output_get (`KismetMathLibrary.Conv_DoubleToVector` 0.5))
      (bind _staticmesh (`/Game/Blueprints/Actors/BinsRubbish.StaticMesh` _output_get))
      (`PrimitiveComponent.SetSimulatePhysics` _staticmesh true)
      (set `PrimitiveComponent.CanCharacterStepUpOn` "ECB_No" _staticmesh))))

(event `Spawn Rubbish`
  (goto _label :!via `Reset`))