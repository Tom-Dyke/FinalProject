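; Delivery tutorial trigger actor that introduces box delivery to the player on day 0.
; On BeginPlay it binds to the player character's new-day event, finds its attached "hero2" manager actor by display name and unhides it.
; The player's first day-0 overlap plays a dialogue message after a short delay and forces the player's BoxSpawner to produce a box.
; The new-day event destroys the manager, then the trigger itself.
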(event `self.ReceiveBeginPlay`
  (bind _asbp_first_person_character (cast `/Game/FirstPerson/Blueprints/BP_FirstPersonCharacter` (`GameplayStatics.GetPlayerCharacter` 0)))
  (bind _output_get (set `self.Player Character` _asbp_first_person_character))
  (add `/Game/FirstPerson/Blueprints/BP_FirstPersonCharacter.NewDay` _output_get (delegate `Day`))
  (for _array_element (`self.GetAttachedActors` true)
    (if (`KismetStringLibrary.EqualEqual_StrStr` (`KismetSystemLibrary.GetDisplayName` _array_element) "hero2")
      (set `self.Manager` _array_element)))
  (`self.SetActorHiddenInGame` (`self.Manager`) false))

(event `Day`
  (params (`Day Number` :type Integer))
  (switch `int` `Day Number`
    (:`Default`
      (`self.K2_DestroyActor` (`self.Manager`))
      (`self.DestroySelf`))))

(event `self.ReceiveActorBeginOverlap`
  (params (OtherActor :type "Actor Object Reference"))
  (if (== OtherActor (`self.Player Character`))
    (switch `int` (`/Game/FirstPerson/Blueprints/BP_FirstPersonCharacter.DayNumber` (`self.Player Character`))
      (:`0`
        (`/Engine/EditorBlueprintResources/StandardMacros.DoOnce` false
          (:`Completed`
            (`KismetSystemLibrary.Delay` 1.0)
            (message `/Game/Blueprints/Interfaces/InteractInterface.Interact` (`self.DialogueComponent`) (`self.Player Character`))
            (`/Game/Blueprints/Actors/SpawnBoxes.Force Box` (`/Game/FirstPerson/Blueprints/BP_FirstPersonCharacter.BoxSpawner` (`self.Player Character`)))))))))

(event `DestroySelf`
  (`KismetSystemLibrary.Delay` 0.5)
  (`self.K2_DestroyActor`))

(fn `UserConstructionScript`)