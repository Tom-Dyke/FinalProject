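; Trigger box that turns the player back in a fog reset once their shift is finished.
; On overlap it plays a cached FadeOut sequence, locks look input, calls FogResetPlayer with a point offset from the box, then reverses the fade.
; It then restores look input and unhides the character's Kjey.
; DoOnce nodes gate the sequence, and the replay gate resets through the character's NewDay event.
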(event `self.ReceiveActorBeginOverlap`
  (params (OtherActor :type "Actor Object Reference"))
  (if (== OtherActor (`GameplayStatics.GetPlayerCharacter` 0))
    (bind _asbp_first_person_character (cast `/Game/FirstPerson/Blueprints/BP_FirstPersonCharacter` OtherActor))
    (bind _output_get (set `self.BP First Person Character` _asbp_first_person_character))
    (if (`/Game/FirstPerson/Blueprints/BP_FirstPersonCharacter.FinishedShift` _output_get)
      (add `/Game/FirstPerson/Blueprints/BP_FirstPersonCharacter.NewDay` (`self.BP First Person Character`) (delegate `Reset Fog`))
      (`/Engine/EditorBlueprintResources/StandardMacros.IsValid` (`self.Sequence Player`)
        (:`Is Valid`
          (`/Engine/EditorBlueprintResources/StandardMacros.DoOnce` false :!label _label
            (:`Completed`
              _)))
        (:`Is Not Valid`
          (`/Engine/EditorBlueprintResources/StandardMacros.DoOnce` false
            (:`Completed`
              (bind (_outactor _returnvalue) (`LevelSequencePlayer.CreateLevelSequencePlayer` (`self.Fade Out`) (make `MovieSceneSequencePlaybackSettings` false (struct) 1.0 0.0 false false false false false false false true)))
              (set `self.Sequence Player` _returnvalue)))))
      (`MovieSceneSequencePlayer.Play` (`self.Sequence Player`))
      (`KismetSystemLibrary.Delay` 2.0)
      (`Controller.SetIgnoreLookInput` (`GameplayStatics.GetPlayerController` 0) true)
      (`/Game/FirstPerson/Blueprints/BP_FirstPersonCharacter.FogResetPlayer` (`self.BP First Person Character`) (+ (`self.K2_GetActorLocation` self) (200.0 0.0 0.0)))
      (`KismetSystemLibrary.Delay` 1.0)
      (`MovieSceneSequencePlayer.PlayReverse` (`self.Sequence Player`))
      (`KismetSystemLibrary.Delay` 1.0)
      (`Controller.SetIgnoreLookInput` (`GameplayStatics.GetPlayerController` 0) false)
      (switch `int` (`/Game/FirstPerson/Blueprints/BP_FirstPersonCharacter.DayNumber` (`self.BP First Person Character`))
        (:`Default`
          (`SceneComponent.SetHiddenInGame` (`/Game/FirstPerson/Blueprints/BP_FirstPersonCharacter.kjey` (`self.BP First Person Character`)) false false))))))

(event `Reset Fog`
  (params (`Day Number` :type Integer))
  (goto _label :!via `Reset`))

(fn `UserConstructionScript`)