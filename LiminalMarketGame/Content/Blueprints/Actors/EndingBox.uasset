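; EndingBox is a trigger actor that teleports the player for the game's ending once the final conditions are met.
; On actor overlap by the player character, it checks BP_FirstPersonCharacter for a finished shift on day four.
; When both hold, it moves the player to its DestLocation, using the controller's current control rotation as the destination rotation.
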(event `self.ReceiveActorBeginOverlap`
  (params (OtherActor :type "Actor Object Reference"))
  (if (== OtherActor (`GameplayStatics.GetPlayerCharacter` 0))
    (bind _asbp_first_person_character (cast `/Game/FirstPerson/Blueprints/BP_FirstPersonCharacter` (`GameplayStatics.GetPlayerCharacter` 0)))
    (if (and (`/Game/FirstPerson/Blueprints/BP_FirstPersonCharacter.FinishedShift` _asbp_first_person_character) (== (`/Game/FirstPerson/Blueprints/BP_FirstPersonCharacter.DayNumber` _asbp_first_person_character) 4))
      (`self.K2_TeleportTo` _asbp_first_person_character (`self.Dest Location`) (`Controller.GetControlRotation` (`GameplayStatics.GetPlayerController` 0))))))

(fn `UserConstructionScript`)