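; Spill actor that presents a day-specific floor mess as a splatter decal with a matching item mesh.
; BeginPlay disables the Box collision and hides the Decal and StaticMesh in game.
; OnSpawn switches on DayNumber, dressing day 3 as a sauce bottle spill and day 4 as a blood splatter with a fillet knife, repositioning the item to fit.
; Nothing in this graph re-enables collision or visibility.
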(event `self.ReceiveBeginPlay`
  (`PrimitiveComponent.SetCollisionEnabled` (`self.Box`) "NoCollision")
  (`SceneComponent.SetHiddenInGame` (`self.Decal`) true false)
  (`SceneComponent.SetHiddenInGame` (`self.StaticMesh`) true false))

(event `OnSpawn`
  (params (`Day Number` :type Integer))
  (bind _decal (`self.Decal`))
  (bind _item (`self.Item`))
  (switch `int` `Day Number`
    (:`3`
      (`DecalComponent.SetDecalMaterial` _decal "/Game/LiminalMarket/Aquired_Assets/Decals/SpillDecals/SauceSplatter.SauceSplatter")
      (`StaticMeshComponent.SetStaticMesh` _item "/Game/MMSupermarket/Products/Mesh/SM_SacueBottle04.SM_SacueBottle04")
      (`SceneComponent.K2_AddLocalOffset` (`self.Item`) (0.0 0.0 -2.0) false false))
    (:`4`
      (`DecalComponent.SetDecalMaterial` _decal "/Game/LiminalMarket/Aquired_Assets/Decals/SpillDecals/BloodSplatter.BloodSplatter")
      (`StaticMeshComponent.SetStaticMesh` _item "/Game/LiminalMarket/FishMongerAssets/Fish_FilletKnife.Fish_FilletKnife")
      (`SceneComponent.K2_SetRelativeTransform` (`self.Item`) (`KismetMathLibrary.MakeTransform` (22.528455 -14.218332 -38.628265) (struct :`Pitch` 90.0 :`Yaw` 20.556045 :`Roll` -24.443956)) false false))))

(fn `UserConstructionScript`)