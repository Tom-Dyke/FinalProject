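; Interactable shop or workplace door that the player opens and closes as part of a day-based shift routine.
; It binds to the first-person character's NewDay event, plays its ActorSequence forward or reversed to set each day's starting state, and resets its DoOnce gates.
; Interaction depends on day, shift completion and key visibility.
; Opening or closing toggles the player's key mesh and clipboard checkboxes, and opening also calls OpenDoors on the player.
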(event `self.ReceiveBeginPlay`
  (bind _asbp_first_person_character (cast `/Game/FirstPerson/Blueprints/BP_FirstPersonCharacter` (`GameplayStatics.GetPlayerCharacter` 0)))
  (add `/Game/FirstPerson/Blueprints/BP_FirstPersonCharacter.NewDay` _asbp_first_person_character (delegate `DayUpdate`))
  (set `/Game/FirstPerson/Blueprints/BP_FirstPersonCharacter.DoorBlueprint` self _asbp_first_person_character))

(event `DayUpdate`
  (params (`Day Number` :type Integer))
  (bind _sequenceplayer (`ActorSequenceComponent.SequencePlayer` (`self.ActorSequence`)))
  (bind _output_get (set `self.Day Number` `Day Number`))
  (switch `int` _output_get
    (:`1`
      (`MovieSceneSequencePlayer.Play` _sequenceplayer :!label _label))
    (:`2`
      (goto _label))
    (:`3`
      (`MovieSceneSequencePlayer.PlayReverse` _sequenceplayer :!label _label_2))
    (:`4`
      (goto _label_2)))
  (`self.Day Reset`))

(event `Day Reset`
  (bind _returnvalue (`WidgetComponent.GetWidget` (`/Game/FirstPerson/Blueprints/BP_FirstPersonCharacter.Widget` (`self.Player Character`))))
  (`|ExecutionSequence`
    (:`then_0`
      (goto _label_5 :!via `Reset`))
    (:`then_1`
      (goto _label_6 :!via `Reset`))))

(event `/Game/Blueprints/Interfaces/InteractInterface.Interact`
  (params (`Player Character` :type "/Game/FirstPerson/Blueprints/BP_FirstPersonCharacter Object Reference"))
  (bind _kjey (`/Game/FirstPerson/Blueprints/BP_FirstPersonCharacter.kjey` `Player Character`))
  (bind _returnvalue (`WidgetComponent.GetWidget` (`/Game/FirstPerson/Blueprints/BP_FirstPersonCharacter.Widget` (`self.Player Character`))))
  (bind _output_get (set `self.Player Character` `Player Character`))
  (switch `int` (`/Game/FirstPerson/Blueprints/BP_FirstPersonCharacter.DayNumber` _output_get)
    (:`2`
      (if (`/Game/FirstPerson/Blueprints/BP_FirstPersonCharacter.FinishedShift` (`self.Player Character`))
        (`/Engine/EditorBlueprintResources/StandardMacros.DoOnce` false
          (:`Completed`
            (`MovieSceneSequencePlayer.PlayReverse` (`ActorSequenceComponent.SequencePlayer` (`self.ActorSequence`)))
            (`SceneComponent.SetHiddenInGame` _kjey false false)
            (bind _asclipboard_widget (cast `/Game/Blueprints/Widgets/ClipboardWidget` _returnvalue :!label _label_3))
            (`CheckBox.SetIsChecked` (`/Game/Blueprints/Widgets/ClipboardWidget.Doors_close` _asclipboard_widget) true)
            (`CheckBox.SetIsChecked` (`/Game/Blueprints/Widgets/ClipboardWidget.Doors` _asclipboard_widget) false)
            (set `self.Doors Closed` true)))))
    (:`3`
      (if (`SceneComponent.bHiddenInGame` _kjey) :!label _label_4
        (if (`/Game/FirstPerson/Blueprints/BP_FirstPersonCharacter.FinishedShift` (`self.Player Character`))
          (`/Engine/EditorBlueprintResources/StandardMacros.DoOnce` false :!label _label_5
            (:`Completed`
              (`MovieSceneSequencePlayer.PlayReverse` (`ActorSequenceComponent.SequencePlayer` (`self.ActorSequence`)))
              (`SceneComponent.SetHiddenInGame` _kjey false false)
              (goto _label_3))))
        (else
          (`/Engine/EditorBlueprintResources/StandardMacros.DoOnce` false :!label _label_6
            (:`Completed`
              (`MovieSceneSequencePlayer.Play` (`ActorSequenceComponent.SequencePlayer` (`self.ActorSequence`)))
              (`SceneComponent.SetHiddenInGame` _kjey true false)
              (`/Game/FirstPerson/Blueprints/BP_FirstPersonCharacter.Open Doors` (`self.Player Character`))
              (bind _asclipboard_widget_2 (cast `/Game/Blueprints/Widgets/ClipboardWidget` _returnvalue))
              (`CheckBox.SetIsChecked` (`/Game/Blueprints/Widgets/ClipboardWidget.Doors` _asclipboard_widget_2) true)
              (`CheckBox.SetIsChecked` (`/Game/Blueprints/Widgets/ClipboardWidget.Doors_close` _asclipboard_widget_2) false)
              (set `self.Doors Closed` false))))))
    (:`4`
      (goto _label_4))))

(fn `UserConstructionScript`)