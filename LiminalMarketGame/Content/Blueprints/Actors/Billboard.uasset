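; Billboard actor whose displayed image changes as in-game days pass.
; On BeginPlay it casts the player to BP_FirstPersonCharacter and binds its Change event to that character's NewDay event.
; Change switches on the day number, swapping the static mesh's first material to a different billboard material on days two through four.
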(event `self.ReceiveBeginPlay`
  (bind _asbp_first_person_character (cast `/Game/FirstPerson/Blueprints/BP_FirstPersonCharacter` (`GameplayStatics.GetPlayerCharacter` 0)))
  (bind _output_get (set `self.As BP First Person Character` _asbp_first_person_character))
  (add `/Game/FirstPerson/Blueprints/BP_FirstPersonCharacter.NewDay` _output_get (delegate `Change`)))

(event `Change`
  (params (`Day Number` :type Integer))
  (switch `int` `Day Number`
    (:`2`
      (`PrimitiveComponent.SetMaterial` (`self.StaticMesh`) 0 "/Game/LiminalMarket/PostersBillboards/billboard1_Mat.billboard1_Mat"))
    (:`3`
      (`PrimitiveComponent.SetMaterial` (`self.StaticMesh`) 0 "/Game/LiminalMarket/PostersBillboards/billboard2_Mat.billboard2_Mat"))
    (:`4`
      (`PrimitiveComponent.SetMaterial` (`self.StaticMesh`) 0 "/Game/LiminalMarket/PostersBillboards/billboard3_Mat.billboard3_Mat"))))

(fn `UserConstructionScript`)