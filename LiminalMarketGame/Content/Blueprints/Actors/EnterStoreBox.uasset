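; Store entrance trigger box that opens and closes the doors by playing the OpenDoor level sequence forward or in reverse.
; Player's NewDay event opens them automatically on early days.
; From day three, overlapping with the key visible before the shift ends hides it, opens the doors and checks the clipboard task.
; With the key hidden, overlap offers a "Close" interaction that restores the key, closes the doors and checks that task.
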(event `CloseDoors`
  (bind _levelsequence (`self.LevelSequence`))
  (`/Engine/EditorBlueprintResources/StandardMacros.IsValid` _levelsequence
    (:`Is Valid`
      (`MovieSceneSequencePlayer.PlayReverse` _levelsequence))
    (:`Is Not Valid`
      (`/Engine/EditorBlueprintResources/StandardMacros.DoOnce` false
        (:`Completed`
          (bind (_outactor _returnvalue) (`LevelSequencePlayer.CreateLevelSequencePlayer` (`self.Open Door`) (make `MovieSceneSequencePlaybackSettings` false (struct) 1.0 0.0 false false false false false false false true)))
          (bind _output_get (set `self.LevelSequence` _returnvalue))
          (`MovieSceneSequencePlayer.PlayReverse` _output_get))))))

(event `OpenDoors`
  (`/Engine/EditorBlueprintResources/StandardMacros.IsValid` (`self.LevelSequence`)
    (:`Is Valid`
      (`MovieSceneSequencePlayer.Play` (`self.LevelSequence`)))
    (:`Is Not Valid`
      (`/Engine/EditorBlueprintResources/StandardMacros.DoOnce` false
        (:`Completed`
          (bind (_outactor _returnvalue) (`LevelSequencePlayer.CreateLevelSequencePlayer` (`self.Open Door`) (make `MovieSceneSequencePlaybackSettings` false (struct) 1.0 0.0 false false false false false false false true)))
          (bind _output_get (set `self.LevelSequence` _returnvalue))
          (`MovieSceneSequencePlayer.Play` _output_get))))))

(event `self.ReceiveBeginPlay`
  (bind _asbp_first_person_character (cast `/Game/FirstPerson/Blueprints/BP_FirstPersonCharacter` (`GameplayStatics.GetPlayerCharacter` 0)))
  (add `/Game/FirstPerson/Blueprints/BP_FirstPersonCharacter.NewDay` _asbp_first_person_character (delegate `UpdateDay`)))

(event `UpdateDay`
  (params (`Day Number` :type Integer))
  (bind _output_get (set `self.Day Number` `Day Number`))
  (if (and (< _output_get 3) (!= _output_get 0))
    (`self.OpenDoors`)))

(event `/Game/Blueprints/Interfaces/InteractInterface.Interact`
  (params (`Player Character` :type "/Game/FirstPerson/Blueprints/BP_FirstPersonCharacter Object Reference"))
  (`SceneComponent.SetHiddenInGame` (`/Game/FirstPerson/Blueprints/BP_FirstPersonCharacter.kjey` `Player Character`) false false)
  (`self.CloseDoors`)
  (bind _asclipboard_widget (cast `/Game/Blueprints/Widgets/ClipboardWidget` (`WidgetComponent.GetWidget` (`/Game/FirstPerson/Blueprints/BP_FirstPersonCharacter.Widget` `Player Character`))))
  (`CheckBox.SetIsChecked` (`/Game/Blueprints/Widgets/ClipboardWidget.Doors_close` _asclipboard_widget) true))

(event `self.ReceiveActorBeginOverlap`
  (params (OtherActor :type "Actor Object Reference"))
  (if (== OtherActor (`GameplayStatics.GetPlayerCharacter` 0))
    (bind _asbp_first_person_character (cast `/Game/FirstPerson/Blueprints/BP_FirstPersonCharacter` (`GameplayStatics.GetPlayerCharacter` 0)))
    (bind _output_get (set `self.First Person Character` _asbp_first_person_character))
    (bind _kjey (`/Game/FirstPerson/Blueprints/BP_FirstPersonCharacter.kjey` _output_get))
    (if (`SceneComponent.bHiddenInGame` _kjey)
      (`/Game/FirstPerson/Blueprints/BP_FirstPersonCharacter.CreateInteractWidget` (`self.First Person Character`) "Close")
      (elif (and (>= (`self.Day Number`) 3) (!= (`/Game/FirstPerson/Blueprints/BP_FirstPersonCharacter.FinishedShift` _output_get) true))
        (`SceneComponent.SetHiddenInGame` _kjey true false)
        (`self.OpenDoors`)
        (bind _asclipboard_widget (cast `/Game/Blueprints/Widgets/ClipboardWidget` (`WidgetComponent.GetWidget` (`/Game/FirstPerson/Blueprints/BP_FirstPersonCharacter.Widget` (`self.First Person Character`)))))
        (`CheckBox.SetIsChecked` (`/Game/Blueprints/Widgets/ClipboardWidget.Doors` _asclipboard_widget) true)))))

(fn `UserConstructionScript`)