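; Spawner actor that drops batches of physics-simulated checkout items at its own transform and registers itself with the first-person character.
; SpawnItems opens a Tick-driven gate through a DoN, and a custom delayed DoN Complete macro spawns items until NumberOfItems is reached.
; Finishing closes the gate and resets both counters for another batch.
; Kill destroys the tracked items, while Leave also resets the spawn cycle.
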(event `self.ReceiveBeginPlay`
  (bind _asbp_first_person_character (cast `/Game/FirstPerson/Blueprints/BP_FirstPersonCharacter` (`GameplayStatics.GetPlayerCharacter` 0)))
  (set `self.BP First Person Character` _asbp_first_person_character)
  (set `/Game/FirstPerson/Blueprints/BP_FirstPersonCharacter.ItemSpawner` self _asbp_first_person_character))

(event `self.ReceiveTick`
  (params (DeltaSeconds :type "Float (single-precision)"))
  (`/Engine/EditorBlueprintResources/StandardMacros.Gate` true :!label _label
    (:`Exit`
      (`self.DoN Complete` (`self.Number of Items`) 0.5 :!label _label_2
        (:`Exit`
          (bind _returnvalue (`|SpawnActorFromClass` "/Game/Blueprints/Actors/CheckoutItems.CheckoutItems_C" (`self.GetTransform`) "Undefined" "OverrideRootScale" null null))
          (`PrimitiveComponent.SetSimulatePhysics` (`/Game/Blueprints/Actors/CheckoutItems.StaticMesh` _returnvalue) true)
          (`KismetArrayLibrary.Array_Add` (`self.ItemsSpawned`) _returnvalue))
        (:`Finished`
          (`|ExecutionSequence` :!label _label_3
            (:`then_0`
              (goto _label :!via `Close`))
            (:`then_1`
              (goto _label_2 :!via `Reset`))
            (:`then_2`
              (goto _label_4 :!via `Reset`))))))))

(event `Spawn Items`
  (`/Engine/EditorBlueprintResources/StandardMacros.Do N` 1 :!label _label_4
    (:`Exit`
      (goto _label :!via `Open`))))

(event `Leave`
  (`self.Kill`)
  (goto _label_3))

(event `Kill`
  (for _array_element (`self.ItemsSpawned`)
    (`/Engine/EditorBlueprintResources/StandardMacros.IsValid` _array_element
      (:`Is Valid`
        (`self.K2_DestroyActor` _array_element))))
  (`KismetArrayLibrary.Array_Clear` (`self.ItemsSpawned`)))

(fn `UserConstructionScript`)