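; Bakery station actor where, from day four, the player delivers the baked good a waiting customer wants.
; It registers with the first-person character, then shows a random order as a spinning mesh (the Roll case is unreachable with RandomInteger(3)).
; On player overlap, a matching item finishes the customer and hides the order.
; Either result clears the carried item, and a mismatch shows a brief, DoOnce-guarded "Wrong Item!" popup.
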(event `self.ReceiveTick`
  (params (DeltaSeconds :type "Float (single-precision)"))
  (bind _staticmesh (`self.StaticMesh`))
  (`SceneComponent.K2_SetRelativeRotation` _staticmesh (`KismetMathLibrary.MakeRotator` (.roll (`SceneComponent.RelativeRotation` _staticmesh)) (.pitch (`SceneComponent.RelativeRotation` _staticmesh)) (+ (.yaw (`SceneComponent.RelativeRotation` _staticmesh)) 1.0)) false false))

(event `self.ReceiveBeginPlay`
  (`BillboardComponent.SetSprite` (`self.SpriteComponent`) null)
  (`SceneComponent.SetHiddenInGame` (`self.StaticMesh`) true false)
  (bind _asbp_first_person_character (cast `/Game/FirstPerson/Blueprints/BP_FirstPersonCharacter` (`GameplayStatics.GetPlayerCharacter` 0)))
  (bind _output_get (set `self.As BP First Person Character` _asbp_first_person_character))
  (set `/Game/FirstPerson/Blueprints/BP_FirstPersonCharacter.BakeryStation` self _output_get))

(event `Bakery Customer`
  (params (Customer :type "/Game/Blueprints/AI/Customer/BP_Customer Object Reference"))
  (bind _as_bp_first_person_character (`self.As BP First Person Character`))
  (bind _staticmesh (`self.StaticMesh`))
  (bind _staticmesh_2 (`self.StaticMesh`))
  (bind _staticmesh_3 (`self.StaticMesh`))
  (bind _staticmesh_4 (`self.StaticMesh`))
  (set `self.Customer` Customer)
  (if (and (`/Game/FirstPerson/Blueprints/BP_FirstPersonCharacter.CustomerWaitingBakery` _as_bp_first_person_character) (>= (`/Game/FirstPerson/Blueprints/BP_FirstPersonCharacter.DayNumber` _as_bp_first_person_character) 4))
    (switch `int` (`KismetMathLibrary.RandomInteger` 3)
      (:`0`
        (`StaticMeshComponent.SetStaticMesh` _staticmesh "/Game/MMSupermarket/Products/Mesh/SM_Baguette.SM_Baguette")
        (`SceneComponent.SetHiddenInGame` _staticmesh false false)
        (set `self.WantedBakedGood` "Baguette")
        (`SceneComponent.SetWorldScale3D` (`self.StaticMesh`) (`KismetMathLibrary.Conv_DoubleToVector` 1.0)))
      (:`1`
        (`StaticMeshComponent.SetStaticMesh` _staticmesh_3 "/Game/MMSupermarket/Products/Mesh/SM_Donut01.SM_Donut01")
        (`SceneComponent.SetHiddenInGame` _staticmesh_3 false false)
        (set `self.WantedBakedGood` "Donut")
        (`SceneComponent.SetWorldScale3D` (`self.StaticMesh`) (`KismetMathLibrary.Conv_DoubleToVector` 2.5)))
      (:`2`
        (`StaticMeshComponent.SetStaticMesh` _staticmesh_4 "/Game/LiminalMarket/Aquired_Assets/Bread/baked-goods/source/baked_goods_pastry-1.baked_goods_pastry-1")
        (`SceneComponent.SetHiddenInGame` _staticmesh_4 false false)
        (set `self.WantedBakedGood` "Croissant")
        (`SceneComponent.SetWorldScale3D` (`self.StaticMesh`) (`KismetMathLibrary.Conv_DoubleToVector` 0.25)))
      (:`3`
        (`StaticMeshComponent.SetStaticMesh` _staticmesh_2 "/Game/LiminalMarket/Aquired_Assets/Bread/game-ready-free-bread-loaf/source/bread_1_mesh.bread_1_mesh")
        (`SceneComponent.SetHiddenInGame` _staticmesh_2 false false)
        (set `self.WantedBakedGood` "Roll")
        (`SceneComponent.SetWorldScale3D` (`self.StaticMesh`) (`KismetMathLibrary.Conv_DoubleToVector` 1.0))))))

(event `self.ReceiveActorBeginOverlap`
  (params (OtherActor :type "Actor Object Reference"))
  (bind _as_bp_first_person_character (`self.As BP First Person Character`))
  (bind _baked_good (`/Game/FirstPerson/Blueprints/BP_FirstPersonCharacter.Baked Good` _as_bp_first_person_character))
  (if (== OtherActor (`GameplayStatics.GetPlayerCharacter` 0))
    (if (>= (`/Game/FirstPerson/Blueprints/BP_FirstPersonCharacter.DayNumber` _as_bp_first_person_character) 4)
      (if (== "None" _baked_good)
        _
        (elif (`/Game/FirstPerson/Blueprints/BP_FirstPersonCharacter.CustomerWaitingBakery` (`self.As BP First Person Character`))
          (if (== _baked_good (`self.WantedBakedGood`))
            (`/Game/FirstPerson/Blueprints/BP_FirstPersonCharacter.FinishCustomerBakery` (`self.As BP First Person Character`) (`self.Customer`))
            (`SceneComponent.SetHiddenInGame` (`self.StaticMesh`) true false)
            (`self.Destroy Connection`)
            (else
              (`self.Destroy Connection`)
              (`self.Wrong Item`))))))))

(event `Destroy Connection`
  (bind _as_bp_first_person_character (`self.As BP First Person Character`))
  (`SceneComponent.SetHiddenInGame` (`/Game/FirstPerson/Blueprints/BP_FirstPersonCharacter.BreadItem` _as_bp_first_person_character) true false)
  (set `/Game/FirstPerson/Blueprints/BP_FirstPersonCharacter.Baked Good` "None" _as_bp_first_person_character))

(event `Wrong Item`
  (`/Engine/EditorBlueprintResources/StandardMacros.DoOnce` false :!label _label
    (:`Completed`
      (`self.Pop-Up`
        (:`then`)
        (:`else`
          (bind _returnvalue (`|CreateWidget` "/Game/Blueprints/Widgets/Pop-UpWidget.Pop-UpWidget_C" null "Wrong Item!"))
          (bind _output_get (set `self.Pop-Up` _returnvalue))
          (`UserWidget.AddToViewport` _output_get 0)
          (`KismetSystemLibrary.Delay` 1.0)
          (`Widget.RemoveFromParent` _output_get)
          (set `self.Pop-Up` null)
          (`self.Reset Widget`))))))

(event `Reset Widget`
  (goto _label :!via `Reset`))

(fn `UserConstructionScript`)