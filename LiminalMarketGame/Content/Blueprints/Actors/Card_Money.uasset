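; Money prop actor that randomly appears as a credit card, cash or coins when play begins.
; BeginPlay rolls a random integer to set MoneyType, then switches on it to assign the matching static mesh and a per-type actor scale.
; Card and cash use negative scales, while coins use a small positive one.
; Tick, overlap and the construction script hold no logic.
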(event `self.ReceiveBeginPlay`
  (switch `int` (`KismetMathLibrary.RandomIntegerInRange` 0 2)
    (:`0`
      (set `self.Money Type` "Card"))
    (:`1`
      (set `self.Money Type` "Cash"))
    (:`2`
      (set `self.Money Type` "Coin")))
  (switch `name` (`self.Money Type`)
    (:`Card`
      (`StaticMeshComponent.SetStaticMesh` (`self.StaticMesh`) "/Game/LiminalMarket/Aquired_Assets/cash/credit_card.credit_card")
      (`self.SetActorScale3D` (`KismetMathLibrary.Conv_DoubleToVector` -7.0)))
    (:`Cash`
      (`StaticMeshComponent.SetStaticMesh` (`self.StaticMesh`) "/Game/LiminalMarket/Aquired_Assets/cash/cash.cash")
      (`self.SetActorScale3D` (`KismetMathLibrary.Conv_DoubleToVector` -10.0)))
    (:`Coin`
      (`StaticMeshComponent.SetStaticMesh` (`self.StaticMesh`) "/Game/LiminalMarket/models/money/Coins.Coins")
      (`self.SetActorScale3D` (`KismetMathLibrary.Conv_DoubleToVector` 0.3)))))

(fn `UserConstructionScript`)