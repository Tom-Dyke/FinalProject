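; EndingScreenBox is a trigger actor that ends play with an ending screen when the player character overlaps it.
; On overlap it plays the FadeOut level sequence, creating and caching the sequence player if needed.
; After a short delay it ignores look input, adds the EndingScreen widget and switches to UI-only input.
; The mouse cursor appears only when the character's UsingController flag is off.
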(event `self.ReceiveActorBeginOverlap`
  (params (OtherActor :type "Actor Object Reference"))
  (bind _returnvalue (`GameplayStatics.GetPlayerController` 0))
  (bind _returnvalue_2 (`GameplayStatics.GetPlayerController` 0))
  (if (== OtherActor (`GameplayStatics.GetPlayerCharacter` 0))
    (bind _asbp_first_person_character (cast `/Game/FirstPerson/Blueprints/BP_FirstPersonCharacter` OtherActor))
    (set `self.BP First Person Character` _asbp_first_person_character)
    (`/Engine/EditorBlueprintResources/StandardMacros.IsValid` (`self.Sequence Player`)
      (:`Is Valid`
        (`/Engine/EditorBlueprintResources/StandardMacros.DoOnce` false
          (:`Completed`
            _)))
      (:`Is Not Valid`
        (`/Engine/EditorBlueprintResources/StandardMacros.DoOnce` false
          (:`Completed`
            (bind (_outactor _returnvalue_3) (`LevelSequencePlayer.CreateLevelSequencePlayer` (`self.Fade Out`) (make `MovieSceneSequencePlaybackSettings` false (struct) 1.5 0.0 false false false false false false false true)))
            (set `self.Sequence Player` _returnvalue_3)))))
    (`MovieSceneSequencePlayer.Play` (`self.Sequence Player`))
    (`KismetSystemLibrary.Delay` 2.0)
    (`Controller.SetIgnoreLookInput` _returnvalue_2 true)
    (`Controller.SetIgnoreMoveInput` _returnvalue_2 false)
    (bind _returnvalue_4 (`|CreateWidget` "/Game/Blueprints/Widgets/EndingScreen.EndingScreen_C"))
    (bind _output_get (set `self.EndingScreen` _returnvalue_4))
    (`UserWidget.AddToViewport` _output_get 0)
    (if (not (`/Game/FirstPerson/Blueprints/BP_FirstPersonCharacter.UsingController` (`self.BP First Person Character`)))
      (set `PlayerController.bShowMouseCursor` true _returnvalue))
    (`WidgetBlueprintLibrary.SetInputMode_UIOnlyEx` _returnvalue _output_get)))

(fn `UserConstructionScript`)