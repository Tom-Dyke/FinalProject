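; A trigger actor, apparently for a rubbish tutorial, that starts a one-time dialogue when the player overlaps it on day 0.
; On BeginPlay it caches the first-person character and unhides an attached manager actor, found by the display name "hero3".
; The overlap checks the player's day number, then calls the dialogue component's interact message after a short delay.
; A DestroySelf event removes the actor after a brief delay.
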(event `self.ReceiveBeginPlay`
  (bind _asbp_first_person_character (cast `/Game/FirstPerson/Blueprints/BP_FirstPersonCharacter` (`GameplayStatics.GetPlayerCharacter` 0)))
  (set `self.Player Character` _asbp_first_person_character)
  (for _array_element (`self.GetAttachedActors` true)
    (if (`KismetStringLibrary.EqualEqual_StrStr` (`KismetSystemLibrary.GetDisplayName` _array_element) "hero3")
      (set `self.Manager` _array_element)))
  (`self.SetActorHiddenInGame` (`self.Manager`) false))

(event `self.ReceiveActorBeginOverlap`
  (params (OtherActor :type "Actor Object Reference"))
  (if (== OtherActor (`self.Player Character`))
    (switch `int` (`/Game/FirstPerson/Blueprints/BP_FirstPersonCharacter.DayNumber` (`self.Player Character`))
      (:`0`
        (`/Engine/EditorBlueprintResources/StandardMacros.DoOnce` false
          (:`Completed`
            (`KismetSystemLibrary.Delay` 1.0)
            (message `/Game/Blueprints/Interfaces/InteractInterface.Interact` (`self.DialogueComponent`) (`self.Player Character`))))))))

(event `DestroySelf`
  (`KismetSystemLibrary.Delay` 0.5)
  (`self.K2_DestroyActor`))

(fn `UserConstructionScript`)