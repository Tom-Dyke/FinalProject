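; Poster actor that changes its artwork as the in-game days progress.
; On BeginPlay it binds to the first-person character's NewDay event and applies the phase-one material for the poster variant selected by its Poster variable.
; When a new day fires, the Change event swaps the mesh material to the phase two or phase three version on days three and four.
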(event `self.ReceiveBeginPlay`
  (bind _asbp_first_person_character (cast `/Game/FirstPerson/Blueprints/BP_FirstPersonCharacter` (`GameplayStatics.GetPlayerCharacter` 0)))
  (bind _output_get (set `self.As BP First Person Character` _asbp_first_person_character))
  (add `/Game/FirstPerson/Blueprints/BP_FirstPersonCharacter.NewDay` _output_get (delegate `Change`))
  (switch `int` (`self.Poster`)
    (:`1`
      (`PrimitiveComponent.SetMaterial` (`self.StaticMesh`) 0 "/Game/LiminalMarket/PostersBillboards/Posters/poster_1_Phase1G_Mat.poster_1_Phase1G_Mat"))
    (:`2`
      (`PrimitiveComponent.SetMaterial` (`self.StaticMesh`) 0 "/Game/LiminalMarket/PostersBillboards/Posters/poster_2_Phase1G_Mat.poster_2_Phase1G_Mat"))))

(event `Change`
  (params (`Day Number` :type Integer))
  (switch `int` (`self.Poster`)
    (:`1`
      (switch `int` `Day Number`
        (:`3`
          (`PrimitiveComponent.SetMaterial` (`self.StaticMesh`) 0 "/Game/LiminalMarket/PostersBillboards/Posters/poster_1_Phase2G_Mat.poster_1_Phase2G_Mat"))
        (:`4`
          (`PrimitiveComponent.SetMaterial` (`self.StaticMesh`) 0 "/Game/LiminalMarket/PostersBillboards/Posters/poster_1_Phase3G_Mat.poster_1_Phase3G_Mat"))))
    (:`2`
      (switch `int` `Day Number`
        (:`3`
          (`PrimitiveComponent.SetMaterial` (`self.StaticMesh`) 0 "/Game/LiminalMarket/PostersBillboards/Posters/poster_2_Phase2G_Mat.poster_2_Phase2G_Mat"))
        (:`4`
          (`PrimitiveComponent.SetMaterial` (`self.StaticMesh`) 0 "/Game/LiminalMarket/PostersBillboards/Posters/poster_2_Phase3G_Mat.poster_2_Phase3G_Mat"))))))

(fn `UserConstructionScript`)