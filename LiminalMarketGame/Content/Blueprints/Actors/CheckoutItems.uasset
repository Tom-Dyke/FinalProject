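; Checkout item actor that shows a random product mesh, presumably for a store checkout.
; On BeginPlay it picks a random mesh from MeshArray, prints its name and enables query and physics collision.
; The beer six-pack and cabbage meshes, matched by object name, keep full scale while all others shrink to a smaller uniform scale.
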(event `self.ReceiveBeginPlay`
  (bind _returnvalue (`KismetSystemLibrary.GetObjectName` (`StaticMeshComponent.StaticMesh` (`self.StaticMesh`))))
  (`StaticMeshComponent.SetStaticMesh` (`self.StaticMesh`) (`KismetArrayLibrary.Array_Random` (`self.Mesh Array`)))
  (`KismetSystemLibrary.PrintString` _returnvalue)
  (if (or (`KismetStringLibrary.EqualEqual_StrStr` _returnvalue "SM_ShashBeer6Pack") (`KismetStringLibrary.EqualEqual_StrStr` _returnvalue "CabbageBigger"))
    (`self.SetActorScale3D` (`KismetMathLibrary.Conv_DoubleToVector` 1.0))
    (else
      (`self.SetActorScale3D` (`KismetMathLibrary.Conv_DoubleToVector` 0.6))))
  (`PrimitiveComponent.SetCollisionEnabled` (`self.StaticMesh`) "QueryAndPhysics"))

(fn `UserConstructionScript`)