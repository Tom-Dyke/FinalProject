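; Bakery item actor that represents a pickup baked good, with its type chosen by the BakedGood variable: baguette, donut, croissant or roll.
; On BeginPlay it switches on that type to set the static mesh, then adjusts scale, or position for the croissant.
; When its PickUpBlueprint component activates, it writes the type into HeldObject on the player's BP_FirstPersonCharacter.
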(event `self.ReceiveBeginPlay`
  (bind _staticmesh (`self.StaticMesh`))
  (switch `name` (`self.BakedGood`)
    (:`Baguette`
      (`StaticMeshComponent.SetStaticMesh` _staticmesh "/Game/MMSupermarket/Products/Mesh/SM_Baguette.SM_Baguette")
      (`self.SetActorScale3D` (`KismetMathLibrary.Conv_DoubleToVector` 1.5)))
    (:`Donut`
      (`StaticMeshComponent.SetStaticMesh` _staticmesh "/Game/MMSupermarket/Products/Mesh/SM_Donut01.SM_Donut01")
      (`self.SetActorScale3D` (`KismetMathLibrary.Conv_DoubleToVector` 7.5)))
    (:`Croissant`
      (`StaticMeshComponent.SetStaticMesh` _staticmesh "/Game/LiminalMarket/Aquired_Assets/Bread/baked-goods/source/baked_goods_pastry-1.baked_goods_pastry-1")
      (`self.K2_SetActorLocation` (+ (`self.K2_GetActorLocation`) (10.0 -10.0 0.0))))
    (:`Roll`
      (`StaticMeshComponent.SetStaticMesh` _staticmesh "/Game/LiminalMarket/Aquired_Assets/Bread/game-ready-free-bread-loaf/source/bread_1_mesh.bread_1_mesh")
      (`self.SetActorScale3D` (`KismetMathLibrary.Conv_DoubleToVector` 1.5)))))

(event `self.PickUpBlueprint.OnComponentActivated`
  (params (Component :type "ActorComponent Object Reference") (bReset :type Boolean))
  (bind _asbp_first_person_character (cast `/Game/FirstPerson/Blueprints/BP_FirstPersonCharacter` (`GameplayStatics.GetPlayerCharacter` 0)))
  (set `/Game/FirstPerson/Blueprints/BP_FirstPersonCharacter.Held Object` (`self.BakedGood`) _asbp_first_person_character))

(fn `UserConstructionScript`)