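; SpawnCustomer is a spawner actor that produces waves of customers, and it registers itself with the first-person player character on BeginPlay.
; SpawnCustomers sets a wave size that grows across days one to four, then NextWave resets the spawn counter.
; Tick drives a delayed DoN macro that spawns customers at the actor's transform until the count is reached, recording each and assigning it a random needed station.
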(event `self.ReceiveBeginPlay`
  (bind _asbp_first_person_character (cast `/Game/FirstPerson/Blueprints/BP_FirstPersonCharacter` (`GameplayStatics.GetPlayerCharacter` 0)))
  (set `/Game/FirstPerson/Blueprints/BP_FirstPersonCharacter.CustomerSpawner` self _asbp_first_person_character))

(event `self.ReceiveTick`
  (params (DeltaSeconds :type "Float (single-precision)"))
  (`self.DoN Complete` (`self.Number of Customers`) 5.0 :!label _label
    (:`Exit`
      (bind _returnvalue (`|SpawnActorFromClass` "/Game/Blueprints/AI/Customer/BP_Customer.BP_Customer_C" (`self.GetTransform`) "AlwaysSpawn" "OverrideRootScale" null null))
      (`KismetArrayLibrary.Array_AddUnique` (`self.CustomersSpawned`) _returnvalue)
      (set `/Game/Blueprints/AI/Customer/BP_Customer.StationNeeded` (`KismetArrayLibrary.Array_Random` (`self.Stations`)) _returnvalue))))

(event `NextWave`
  (goto _label :!via `Reset`))

(event `SpawnCustomers`
  (params (`Day Number` :type Integer))
  (switch `int` `Day Number`
    (:`1`
      (set `self.Number of Customers` 5)
      (`self.NextWave`))
    (:`2`
      (set `self.Number of Customers` 7)
      (`self.NextWave`))
    (:`3`
      (set `self.Number of Customers` 9)
      (`self.NextWave`))
    (:`4`
      (set `self.Number of Customers` 11)
      (`self.NextWave`))))

(fn `UserConstructionScript`)