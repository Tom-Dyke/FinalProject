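; Possessable cursor-driven pawn for a checkout station, where the player serves a customer's items and takes payment.
; Mouse or left stick drives traces that drag physics objects via a PhysicsHandle and show hover descriptions keyed by mesh name.
; Once Zoned, it spawns random money with a matching indicator and waits for card scan or drawer deposit.
; Payment or cancel hands control back to the character, except on day 0, which runs dialogue.
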(event `InputVectorAxis|Gamepad_Left2D`
  (params (AxisValue :type "Vector Structure"))
  (bind (_x _y) (`KismetMathLibrary.BreakVector3f` AxisValue))
  (bind (_locationx _locationy) (`PlayerController.GetMousePosition` (`GameplayStatics.GetPlayerController` 0)))
  (if (not (`KismetMathLibrary.Vector_IsNearlyZero` AxisValue 0.1))
    (`KismetSystemLibrary.PrintString` (`KismetStringLibrary.Concat_StrStr` "X =" (`KismetStringLibrary.Conv_DoubleToString` _x) "Y =" (`KismetStringLibrary.Conv_DoubleToString` _y)))
    (`PlayerController.SetMouseLocation` (`GameplayStatics.GetPlayerController` 0) (`KismetMathLibrary.Round` (+ (* _x 10.0) _locationx)) (`KismetMathLibrary.Round` (- _locationy (* _y 10.0))))))

(event `OnPay`
  (bind _cardmoney (`self.CardMoney`))
  ;[1 1 1] Money
  (`self.Spawn Money`)
  (`/Engine/EditorBlueprintResources/StandardMacros.IsValid` _cardmoney
    (:`Is Valid`
      (switch `name` (`/Game/Blueprints/Actors/Card_Money.Money Type` _cardmoney)
        (:`Card`
          (if (`/Game/Blueprints/Actors/Card_Money.Scanned` _cardmoney)
            (`self.K2_DestroyActor` (`self.CardMoney`))
            (`self.SetActorHiddenInGame` (`self.MoneyHighlight`) true)
            (`KismetSystemLibrary.Delay` 1.0)
            (switch `int` (`/Game/FirstPerson/Blueprints/BP_FirstPersonCharacter.DayNumber` (`self.Unposses Character`)) :!label _label
              (:`Default`
                (`self.On Unpossess`))
              (:`0`
                (`self.Trigger Thing`)))))
        (:`Cash`
          (if (`/Game/Blueprints/Actors/Card_Money.In-Drawer` (`self.CardMoney`)) :!label _label_2
            (`self.K2_DestroyActor` (`self.CardMoney`))
            (`self.SetActorHiddenInGame` (`self.MoneyHighlight`) true)
            (`KismetSystemLibrary.Delay` 1.0)
            (goto _label)))
        (:`Coin`
          (goto _label_2))))))

(event `Reset Money`
  ;[1 1 1] Money
  (goto _label_3 :!via `Reset`))

(event `Spawn Money`
  ;[1 1 1] Money
  (`/Engine/EditorBlueprintResources/StandardMacros.DoOnce` false :!label _label_3
    (:`Completed`
      (bind _returnvalue (`|SpawnActorFromClass` "/Game/Blueprints/Actors/Card_Money.Card_Money_C" (`self.GetTransform` (`self.Spawn Items`)) "Undefined" "OverrideRootScale" null (`KismetArrayLibrary.Array_Random` (`self.Money`)) null))
      (bind _output_get (set `self.CardMoney` _returnvalue))
      (`PrimitiveComponent.SetSimulatePhysics` (`/Game/Blueprints/Actors/Card_Money.StaticMesh` _returnvalue) true)
      (bind _outactors (`GameplayStatics.GetAllActorsOfClassWithTag` "/Game/Blueprints/Actors/MoneyIndicator.MoneyIndicator_C" "Indicator"))
      (for _array_element _outactors
        (if (== (`/Game/Blueprints/Actors/MoneyIndicator.Money` _array_element) (`/Game/Blueprints/Actors/Card_Money.Money Type` _output_get))
          (set `self.MoneyHighlight` _array_element)))
      (`self.SetActorHiddenInGame` (`self.MoneyHighlight`) false)
      (`self.Trigger Thing`))))

(event `CreateHover`
  (bind (_worldlocation _worlddirection) (`PlayerController.DeprojectMousePositionToWorld` (`GameplayStatics.GetPlayerController` 0)))
  (if (`self.Able to Create`)
    (bind (_outhit _returnvalue) (`KismetSystemLibrary.LineTraceSingle` :`Start` _worldlocation :`End` (+ _worldlocation (* _worlddirection 1000.0)) :`TraceChannel` "TraceTypeQuery1" :`DrawDebugType` "ForOneFrame" :`DrawTime` 0.0))
    (if _returnvalue
      (bind (_bblockinghit _binitialoverlap _time _distance _location _impactpoint _normal _impactnormal _physmat _hitactor _hitcomponent) (`GameplayStatics.BreakHitResult` _outhit))
      (set `self.Hit Component Hover` _hitactor)
      (if (`|EnumEquality` (`SceneComponent.Mobility` _hitcomponent) (enumliteral `EComponentMobility` "Movable"))
        (bind _output_get (set `self.Hover Component` _hitactor))
        (if (== _output_get (`self.Hit Component Hover`))
          (`KismetSystemLibrary.Delay` 0.9)
          (if (== (`self.Hover Component`) (`self.Hit Component Hover`))
            (`self.HoverWidget`
              (:`then`
                (bind _ashover_widget (cast `/Game/Blueprints/Widgets/HoverWidget` (`self.HoverWidget`)))
                (bind (_title _description) (`self.GetItemDescription` (`self.Hover Component`)))
                (set `/Game/Blueprints/Widgets/HoverWidget.TitleText` _title _ashover_widget)
                (set `/Game/Blueprints/Widgets/HoverWidget.DescriptionText` _description _ashover_widget))
              (:`else`
                (bind (_title_2 _description_2) (`self.GetItemDescription` (`self.Hover Component`)))
                (bind _returnvalue_2 (`|CreateWidget` "/Game/Blueprints/Widgets/HoverWidget.HoverWidget_C" null _title_2 _description_2))
                (bind _output_get_2 (set `self.HoverWidget` _returnvalue_2))
                (`UserWidget.AddToViewport` _output_get_2 0)))
            (else
              (bind _hoverwidget (`self.HoverWidget` :!label _label_4)
                (:`then`
                  (`Widget.RemoveFromParent` _hoverwidget)
                  (set `self.HoverWidget` null))
                (:`else`))))
          (else
            (goto _label_4)))
        (else
          (goto _label_4))))))

(event `EnhancedInput|/Game/Blueprints/Inputs/IA_Interact`
  (params (ActionValue :type Boolean) (ElapsedSeconds :type "Float (double-precision)") (TriggeredSeconds :type "Float (double-precision)") (InputAction :type "InputAction Object Reference" :default "/Game/Blueprints/Inputs/IA_Interact.IA_Interact"))
  (bind _grab_mode (`self.Grab Mode`))
  (bind (_worldlocation _worlddirection) (`PlayerController.DeprojectMousePositionToWorld` (`GameplayStatics.GetPlayerController` 0)))
  (bind _togglehold (`/Game/FirstPerson/Blueprints/BP_FirstPersonCharacter.ToggleHold` (`self.Unposses Character`)))
  (:`Triggered`
    (if _togglehold :!label _label_5
      (if _grab_mode :!label _label_6
        (set `self.Grabbed` true)
        (bind (_outhit _returnvalue) (`KismetSystemLibrary.LineTraceSingle` _worldlocation (+ _worldlocation (* _worlddirection 1000.0)) "TraceTypeQuery1" false (`self.GetAttachedActors` (`self.GetAttachParentActor`) true false) "None" true (struct :`R` 1.0 :`A` 1.0) (struct :`G` 1.0 :`A` 1.0) 0.0))
        (if _returnvalue
          (bind (_bblockinghit _binitialoverlap _time _distance _location _impactpoint _normal _impactnormal _physmat _hitactor _hitcomponent) (`GameplayStatics.BreakHitResult` _outhit))
          (set `self.Hit Component` _hitcomponent)
          (if (`|EnumEquality` (`SceneComponent.Mobility` _hitcomponent) (enumliteral `EComponentMobility` "Movable"))
            (bind (_bblockinghit_2 _binitialoverlap_2 _time_2 _distance_2 _location_2 _impactpoint_2 _normal_2 _impactnormal_2 _physmat_2 _hitactor_2 _hitcomponent_2) (`GameplayStatics.BreakHitResult` _outhit))
            (set `self.Initial Distance` _distance_2)
            (bind _output_get (set `self.Grabbed Component` _hitcomponent_2))
            (`PhysicsHandleComponent.GrabComponentAtLocation` (`self.PhysicsHandle`) _output_get "None" _location_2)
            (set `self.Grab Location` (`KismetMathLibrary.InverseTransformLocation` (`SceneComponent.K2_GetComponentToWorld` (`self.Grabbed Component`)) _location_2)))))))
  (:`Started`
    (if _togglehold
      _
      (elif (`self.Grabbed`)
        (if _grab_mode :!label _label_7
          (set `self.Grabbed Component` null :!label _label_8)
          (`PhysicsHandleComponent.ReleaseComponent` (`self.PhysicsHandle`))
          (set `self.Grabbed` false))
        (else
          (goto _label_6)))))
  (:`Ongoing`
    (goto _label_5))
  (:`Canceled`
    (if _togglehold :!label _label_9
      (goto _label_7)))
  (:`Completed`
    (goto _label_9)))

(event `Release`
  (goto _label_8))

(event `ForceExit`
  (bind _returnvalue (`GameplayStatics.GetPlayerController` 0))
  (bind _hoverwidget (`self.HoverWidget`))
  (bind _unposses_character (`self.Unposses Character`))
  (set `self.Able to Create` false :!label _label_10)
  (for _array_element (`self.GetAttachedActors` true)
    (bind _asspawn_items (cast `/Game/Blueprints/Actors/SpawnItems` _array_element))
    (`/Game/Blueprints/Actors/SpawnItems.Leave` _asspawn_items))
  (`PrimitiveComponent.SetCollisionEnabled` (`self.GetComponentByClass` (`self.GetAttachParentActor`) "/Script/Engine.BoxComponent") "QueryAndProbe")
  (set `self.Scanned` false)
  (set `self.Zoned` false)
  (set `self.Grab Mode` false)
  (set `PlayerController.bShowMouseCursor` false _returnvalue)
  (`/Game/FirstPerson/Blueprints/BP_FirstPersonCharacter.ToggleTrace` _unposses_character)
  (`/Game/FirstPerson/Blueprints/BP_FirstPersonCharacter.Served` _unposses_character)
  (set `/Game/FirstPerson/Blueprints/BP_FirstPersonCharacter.CustomerWaiting` false _unposses_character)
  (`self.Release`)
  (`self.Reset Money`)
  (`Controller.UnPossess` _returnvalue)
  (`Controller.Possess` _returnvalue _unposses_character)
  (`WidgetBlueprintLibrary.SetFocusToGameViewport`)
  (`WidgetBlueprintLibrary.SetInputMode_GameOnly` (`GameplayStatics.GetPlayerController` 0))
  (`/Game/FirstPerson/Blueprints/BP_FirstPersonCharacter.Update Game Stats` _unposses_character "Customer")
  (`/Engine/EditorBlueprintResources/StandardMacros.IsValid` _hoverwidget
    (:`Is Valid`
      (`Widget.RemoveFromParent` _hoverwidget))))

(event `On Unpossess`
  (goto _label_10))

(event `self.ReceiveTick`
  (params (DeltaSeconds :type "Float (single-precision)"))
  (bind (_worldlocation _worlddirection) (`PlayerController.DeprojectMousePositionToWorld` (`GameplayStatics.GetPlayerController` 0)))
  (bind _returnvalue (+ _worldlocation (* _worlddirection (`self.Initial Distance`))))
  (`|ExecutionSequence`
    (:`then_0`
      (if (`self.Zoned`)
        (`self.OnPay`)))
    (:`then_1`
      (if (`self.Grab Mode`)
        (`self.CreateHover`)
        (`/Engine/EditorBlueprintResources/StandardMacros.IsValid` (`self.Grabbed Component`)
          (:`Is Valid`
            (`PhysicsHandleComponent.SetTargetLocation` (`self.PhysicsHandle`) _returnvalue)
            (`KismetSystemLibrary.DrawDebugLine` (`KismetMathLibrary.TransformLocation` (`SceneComponent.K2_GetComponentToWorld` (`self.Grabbed Component`)) (`self.Grab Location`)) _returnvalue (struct :`R` 1.0 :`G` 0.489921 :`B` 0.044729 :`A` 1.0))))))))

(event `EnhancedInput|/Game/Blueprints/Inputs/IA_Cancel`
  (params (ActionValue :type Boolean) (ElapsedSeconds :type "Float (double-precision)") (TriggeredSeconds :type "Float (double-precision)") (InputAction :type "InputAction Object Reference" :default "/Game/Blueprints/Inputs/IA_Cancel.IA_Cancel"))
  (bind _returnvalue (`GameplayStatics.GetPlayerController` 0))
  (bind _unposses_character (`self.Unposses Character`))
  (bind _hoverwidget (`self.HoverWidget`))
  (:`Started`
    (if (not (== (`/Game/FirstPerson/Blueprints/BP_FirstPersonCharacter.DayNumber` (`self.Unposses Character`)) 0))
      (`|ExecutionSequence`
        (:`then_0`
          (set `self.Able to Create` false)
          (set `self.Scanned` false)
          (set `self.Zoned` false)
          (set `self.Grab Mode` false)
          (set `PlayerController.bShowMouseCursor` false _returnvalue)
          (`/Game/FirstPerson/Blueprints/BP_FirstPersonCharacter.ToggleTrace` _unposses_character)
          (`self.Release`)
          (`self.Reset Money`)
          (`Controller.UnPossess` _returnvalue)
          (`Controller.Possess` _returnvalue _unposses_character)
          (`WidgetBlueprintLibrary.SetFocusToGameViewport`)
          (`WidgetBlueprintLibrary.SetInputMode_GameOnly` (`GameplayStatics.GetPlayerController` 0))
          (`/Engine/EditorBlueprintResources/StandardMacros.IsValid` _hoverwidget
            (:`Is Valid`
              (`Widget.RemoveFromParent` _hoverwidget))))
        (:`then_1`
          (for _array_element (`self.GetAttachedActors` true)
            (bind _asspawn_items (cast `/Game/Blueprints/Actors/SpawnItems` _array_element))
            (`/Game/Blueprints/Actors/SpawnItems.Leave` _asspawn_items))
          (set `self.Grabbed Component` null)
          (`PhysicsHandleComponent.ReleaseComponent` (`self.PhysicsHandle`))
          (set `self.Grabbed` false)
          (`PrimitiveComponent.SetCollisionEnabled` (`self.GetComponentByClass` (`self.GetAttachParentActor`) "/Script/Engine.BoxComponent") "QueryAndProbe"))))))

(event `On Possess`
  (params (`Unposses Character` :type "/Game/FirstPerson/Blueprints/BP_FirstPersonCharacter Object Reference"))
  (bind _unposses_character (`self.Unposses Character`))
  (bind _output_get (set `self.Unposses Character` `Unposses Character`))
  (set `self.Grab Mode` true)
  (set `PlayerController.bShowMouseCursor` true (`GameplayStatics.GetPlayerController` 0))
  (set `self.Able to Create` true)
  (for _array_element (`self.GetAttachedActors` true)
    (bind _asspawn_items (cast `/Game/Blueprints/Actors/SpawnItems` _array_element)
      (:`then`
        (`/Game/Blueprints/Actors/SpawnItems.Spawn Items` _asspawn_items)
        (set `self.Spawn Items` _asspawn_items))
      (:`CastFailed`
        (bind _ascollection_box_blueprint (cast `/Game/Blueprints/Actors/CollectionBoxBlueprint` _array_element)
          (:`then`
            (set `/Game/Blueprints/Actors/CollectionBoxBlueprint.Player Character Ref` (`self.Unposses Character`) _ascollection_box_blueprint))
          (:`CastFailed`
            (bind _asscanner_box_blueprint (cast `/Game/Blueprints/Actors/ScannerBoxBlueprint` _array_element))
            (set `/Game/Blueprints/Actors/ScannerBoxBlueprint.Player Ref` (`self.Unposses Character`) _asscanner_box_blueprint))))))
  (`WidgetBlueprintLibrary.SetInputMode_GameAndUIEx` (`GameplayStatics.GetPlayerController` 0) (`/Game/FirstPerson/Blueprints/BP_FirstPersonCharacter.HUDRef` _output_get) "DoNotLock" false true)
  (add `/Game/FirstPerson/Blueprints/BP_FirstPersonCharacter.EndShift` _unposses_character (`|CreateDelegate` :!event `ForceExit`))
  (if (== (`/Game/FirstPerson/Blueprints/BP_FirstPersonCharacter.DayNumber` _unposses_character) 0)
    (`KismetSystemLibrary.Delay` 0.5)
    (`/Game/Blueprints/Components/DialogueComponent.StartDialogue` (`self.DialogueComponent`))))

(event `Trigger Thing`
  (`self.ProgressDialogue`))

(fn `GetItemDescription`
  (params (HoveredActor :type "Actor Object Reference") (Description1 :type Text))
  (returns (Title :type Text) (Description :type Text))
  (bind _returnvalue (`self.GetComponentByClass` HoveredActor "/Script/Engine.StaticMeshComponent"))
  (`/Engine/EditorBlueprintResources/StandardMacros.IsValid` HoveredActor
    (:`Is Valid`
      (`/Engine/EditorBlueprintResources/StandardMacros.IsValid` _returnvalue
        (:`Is Valid`
          (switch `string` (`KismetSystemLibrary.GetObjectName` (`StaticMeshComponent.StaticMesh` _returnvalue))
            (:`pumpkin`
              (return "Pumpkin" "This is a pumpkin you idiot"))
            (:`SM_Watermelon`
              (return "Watermelon" "MMM tasty watermelon"))
            (:`CabbageBigger`
              (return "Cabbage" "A regular sized cabbage"))
            (:`SM_Banana_01`
              (return "Banana" "Bananananananananana"))
            (:`SM_COD`
              (return "Cod" "The fish not the game you stupid"))
            (:`SM_PackagedMeat01`
              (return "Meat" "Definitely normal meat, not suspicious at all"))
            (:`SM_CP2WashPowder2`
              (return "Washing Powder" "What? You've never seen washing powder before?"))
            (:`SM_CP1Spray3`
              (return "Cleaning Spray" "We go though alot of this in a week"))
            (:`SM_CP3Shampoo01`
              (return "Shampoo" "WARNING: DO NOT APPLY TO HAIR"))
            (:`SM_SPTissue2`
              (return "Tissues" "Hope you don't have any t'issues with this product"))
            (:`SM_CFCereal1`
              (return "Cereal" "Provides boundless sugary energy (for about 5 minutes)"))
            (:`SM_Packet1_2_Chips`
              (return "Crisps" "Now with 10% less toenail clippings!"))
            (:`SM_PAPasta1`
              (return "Pasta" "I hope you're feeling saucy"))
            (:`SM_CarnaroliRice`
              (return "Rice" "I'm the rice guy"))
            (:`SM_CookingOil_Small`
              (return "Cooking Oil" "This company accepts no responsibility if its product was used to consume others"))
            (:`SM_ShashBeer6Pack`
              (return "6-Pack Beer" "The reason for your parents divorce"))
            (:`credit_card`
              (return "Credit Card" "Goes to the card scanner"))
            (:`cash`
              (return "Cash" "Goes into the cash register"))
            (:`Coins`
              (return "Coin" "Goes into the money pot"))))))))

(fn `UserConstructionScript`)