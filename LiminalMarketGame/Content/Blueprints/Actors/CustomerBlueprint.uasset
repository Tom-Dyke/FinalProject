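; CustomerBlueprint is an actor that signals whether a customer is present by swapping the material on its Cube component.
; NewCustomer plays the Checkout sound and applies the Cust1 material, while NoCustomer applies the Cust material.
; Unconnected nodes for spawning a Women1 actor at a fixed transform and destroying it remain in the graph but never run.
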(event `NewCustomer`
  (`GameplayStatics.PlaySound2D` "/Game/Sounds/events/checkout.checkout" 1.0 1.0 0.0 null null)
  (`PrimitiveComponent.SetMaterial` (`self.Cube`) 0 "/Game/LiminalMarket/Created_assets/texturemats/cust1.cust1"))

(event `NoCustomer`
  (`PrimitiveComponent.SetMaterial` (`self.Cube`) 0 "/Game/LiminalMarket/Created_assets/texturemats/cust.cust"))

(fn `UserConstructionScript`)