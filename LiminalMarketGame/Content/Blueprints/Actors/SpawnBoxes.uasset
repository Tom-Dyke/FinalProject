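; Delivery spawner actor that drops physics restock boxes at its own location when enough store shelves are empty.
; It caches shelf components at BeginPlay, gathers empty ones on a delayed Tick and, past a threshold outside debug mode, flags all shelves as spawning.
; A delayed loop macro staggers one aisle-specific box per empty shelf, with sound and player signal-material changes.
; An empty box list triggers a one-shot delivery reset and delayed flag clearing.
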(event `self.ReceiveBeginPlay`
  (bind _asbp_first_person_character (cast `/Game/FirstPerson/Blueprints/BP_FirstPersonCharacter` (`GameplayStatics.GetPlayerCharacter` 0)))
  (set `/Game/FirstPerson/Blueprints/BP_FirstPersonCharacter.BoxSpawner` self _asbp_first_person_character)
  (bind _outactors (`GameplayStatics.GetAllActorsOfClass` "/Script/Engine.StaticMeshActor"))
  (for _array_element _outactors
    (bind _returnvalue (`self.GetComponentByClass` _array_element "/Game/Blueprints/Components/ShelfBlueprint.ShelfBlueprint_C"))
    (if (`KismetSystemLibrary.IsValid` _returnvalue)
      (`KismetArrayLibrary.Array_Add` (`self.Shelves`) _returnvalue))))

(event `self.ReceiveTick`
  (params (DeltaSeconds :type "Float (single-precision)"))
  (`self.CheckFinished`)
  (`KismetSystemLibrary.Delay` 5.0)
  (for _array_element (`self.Shelves`)
    (if (`/Game/Blueprints/Components/ShelfBlueprint.Shelf Empty` _array_element)
      (if (== (`KismetArrayLibrary.Array_Find` (`self.Empty Shelves`) _array_element) -1)
        (`KismetArrayLibrary.Array_Add` (`self.Empty Shelves`) _array_element))))
  (if (>= (`KismetArrayLibrary.Array_Length` (`self.Empty Shelves`)) 15)
    (bind _asbp_first_person_character (cast `/Game/FirstPerson/Blueprints/BP_FirstPersonCharacter` (`GameplayStatics.GetPlayerCharacter` 0)))
    (if (not (`/Game/FirstPerson/Blueprints/BP_FirstPersonCharacter.Debug Mode` _asbp_first_person_character))
      (`self.Spawn Boxes`))))

(event `Spawn Boxes`
  (for _array_element (`self.Shelves`)
    (set `/Game/Blueprints/Components/ShelfBlueprint.Spawing?` true _array_element))
  (bind _asbp_first_person_character (cast `/Game/FirstPerson/Blueprints/BP_FirstPersonCharacter` (`GameplayStatics.GetPlayerCharacter` 0)))
  (`PrimitiveComponent.SetMaterial` (`/Game/FirstPerson/Blueprints/BP_FirstPersonCharacter.DeliverySignal` _asbp_first_person_character) 0 "/Game/LiminalMarket/models/texturemats/cust2.cust2")
  (`GameplayStatics.PlaySound2D` "/Game/LiminalMarket/sounds/events/delivery.delivery" 1.0 1.0 0.0 null null)
  (bind _array_element_2 (`self.For Each Loop With Delay` (`self.Empty Shelves`) 0.5)
    (:`Loop Body`
      (bind _returnvalue (`|SpawnActorFromClass` "/Game/Blueprints/Actors/DeliveryBoxes.DeliveryBoxes_C" (`self.GetTransform`) "Undefined" "OverrideRootScale" null (`/Game/Blueprints/Components/ShelfBlueprint.AisleName` _array_element_2) null))
      (bind _staticmesh (`/Game/Blueprints/Actors/DeliveryBoxes.StaticMesh` _returnvalue))
      (`PrimitiveComponent.SetSimulatePhysics` _staticmesh true)
      (set `PrimitiveComponent.CanCharacterStepUpOn` "ECB_No" _staticmesh)
      (`KismetArrayLibrary.Array_Add` (`self.Spawned Boxes`) _returnvalue)
      (set `/Game/Blueprints/Actors/DeliveryBoxes.SpawnBoxesRef` self _returnvalue))
    (:`Completed`
      (bind _asbp_first_person_character_2 (cast `/Game/FirstPerson/Blueprints/BP_FirstPersonCharacter` (`GameplayStatics.GetPlayerCharacter` 0)))
      (`PrimitiveComponent.SetMaterial` (`/Game/FirstPerson/Blueprints/BP_FirstPersonCharacter.DeliverySignal` _asbp_first_person_character_2) 0 "/Game/LiminalMarket/models/texturemats/cust1.cust1"))))

(event `CheckFinished`
  (if (`KismetArrayLibrary.Array_IsEmpty` (`self.Spawned Boxes`))
    (`/Engine/EditorBlueprintResources/StandardMacros.DoOnce` false :!label _label
      (:`Completed`
        (bind _asbp_first_person_character (cast `/Game/FirstPerson/Blueprints/BP_FirstPersonCharacter` (`GameplayStatics.GetPlayerCharacter` 0)))
        (`PrimitiveComponent.SetMaterial` (`/Game/FirstPerson/Blueprints/BP_FirstPersonCharacter.DeliverySignal` _asbp_first_person_character) 0 "/Game/LiminalMarket/models/texturemats/cust.cust")
        (`/Game/FirstPerson/Blueprints/BP_FirstPersonCharacter.ResetDelivery` _asbp_first_person_character 60.0)
        (`KismetSystemLibrary.Delay` 30.0)
        (for _array_element (`self.Shelves`)
          (set `/Game/Blueprints/Components/ShelfBlueprint.Spawing?` false _array_element))))
    (else
      (goto _label :!via `Reset`))))

(fn `UserConstructionScript`)