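; Delivery box actor that takes a random product category and can be picked up by the first-person player.
; On BeginPlay it picks a name from BoxNames, randomly enlarges the mesh per axis and sets the matching category material.
; Activating PickUpBlueprint stores the category and box on the player character and prints the category.
; Washing, cleaning, fridge, frozen and bathroom material setters exist but are unwired.
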(event `self.ReceiveBeginPlay`
  (bind _staticmesh (`self.StaticMesh`))
  (bind _staticmesh_2 (`self.StaticMesh`))
  (bind (_returnvalue_x _returnvalue_y _returnvalue_z) (`KismetMathLibrary.BreakVector` (`SceneComponent.K2_GetComponentScale` _staticmesh_2)))
  (bind _output_get (set `self.ChosenBox` (`|GetArrayItem` (`self.BoxNames`) (`KismetMathLibrary.RandomIntegerInRange` 0 11))))
  (`SceneComponent.SetWorldScale3D` _staticmesh_2 (`KismetMathLibrary.MakeVector` (+ _returnvalue_x (`KismetMathLibrary.RandomFloatInRange` 5.0 50.0)) (+ _returnvalue_y (`KismetMathLibrary.RandomFloatInRange` 5.0 25.0)) (+ _returnvalue_z (`KismetMathLibrary.RandomFloatInRange` 5.0 75.0))))
  (switch `name` _output_get
    (:`Fruit`
      (`PrimitiveComponent.SetMaterial` _staticmesh 0 "/Game/LiminalMarket/Aquired_Assets/Other/cardboard-box/textures/CardboardBox_LP_lambert1_AlbedoTransparencyfruit_Mat.CardboardBox_LP_lambert1_AlbedoTransparencyfruit_Mat"))
    (:`Veg`
      (`PrimitiveComponent.SetMaterial` _staticmesh 0 "/Game/LiminalMarket/Aquired_Assets/Other/cardboard-box/textures/CardboardBox_LP_lambert1_AlbedoTransparencyveg_Mat.CardboardBox_LP_lambert1_AlbedoTransparencyveg_Mat"))
    (:`Snacks`
      (`PrimitiveComponent.SetMaterial` _staticmesh 0 "/Game/LiminalMarket/Aquired_Assets/Other/cardboard-box/textures/CardboardBox_LP_lambert1_AlbedoTransparencysnacks_Mat.CardboardBox_LP_lambert1_AlbedoTransparencysnacks_Mat"))
    (:`Meat`
      (`PrimitiveComponent.SetMaterial` _staticmesh 0 "/Game/LiminalMarket/Aquired_Assets/Other/cardboard-box/textures/CardboardBox_LP_lambert1_AlbedoTransparencymeat_Mat.CardboardBox_LP_lambert1_AlbedoTransparencymeat_Mat"))
    (:`Everyday`
      (`PrimitiveComponent.SetMaterial` _staticmesh 0 "/Game/LiminalMarket/Aquired_Assets/Other/cardboard-box/textures/CardboardBox_LP_lambert1_AlbedoTransparencyEveryday_Mat.CardboardBox_LP_lambert1_AlbedoTransparencyEveryday_Mat"))
    (:`Cans`
      (`PrimitiveComponent.SetMaterial` _staticmesh 0 "/Game/LiminalMarket/Aquired_Assets/Other/cardboard-box/textures/CardboardBox_LP_lambert1_AlbedoTransparencycans_Mat.CardboardBox_LP_lambert1_AlbedoTransparencycans_Mat"))
    (:`Alcohol`
      (`PrimitiveComponent.SetMaterial` _staticmesh 0 "/Game/LiminalMarket/Aquired_Assets/Other/cardboard-box/textures/CardboardBox_LP_lambert1_AlbedoTransparencyalcohol_Mat.CardboardBox_LP_lambert1_AlbedoTransparencyalcohol_Mat"))))

(event `self.PickUpBlueprint.OnComponentActivated`
  (params (Component :type "ActorComponent Object Reference") (bReset :type Boolean))
  (bind _chosenbox (`self.ChosenBox`))
  (bind _asbp_first_person_character (cast `/Game/FirstPerson/Blueprints/BP_FirstPersonCharacter` (`GameplayStatics.GetPlayerCharacter` 0)))
  (set `/Game/FirstPerson/Blueprints/BP_FirstPersonCharacter.Held Object` _chosenbox _asbp_first_person_character)
  (set `/Game/FirstPerson/Blueprints/BP_FirstPersonCharacter.HeldBox` self _asbp_first_person_character)
  (`KismetSystemLibrary.PrintString` (`KismetStringLibrary.Conv_NameToString` _chosenbox)))

(fn `UserConstructionScript`)