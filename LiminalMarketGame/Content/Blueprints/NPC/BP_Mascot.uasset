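; Mascot NPC actor that jump-scares the player during shifts.
; Teleport event, in shift-time windows varying by day, moves it to a random preset spot in front of the player, found via local-space X, swapping pose and material.
; While overlapped, gated Tick checks proximity, then drops the player far below with muted audio for several seconds before returning them.
; The mascot returns to its original spot and look; DoOnce resets re-arm both triggers.
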(event `self.ReceiveBeginPlay`
  (bind _asbp_first_person_character (cast `/Game/FirstPerson/Blueprints/BP_FirstPersonCharacter` (`GameplayStatics.GetPlayerCharacter` 0)))
  (set `self.Player Character` _asbp_first_person_character))

(event `Teleport`
  (params (`Player Character` :type "/Game/FirstPerson/Blueprints/BP_FirstPersonCharacter Object Reference") (`Day Number` :type Integer))
  (bind _mesh (`self.Mesh`))
  (bind _viablelocations (`self.ViableLocations`))
  (bind _outitem (`KismetArrayLibrary.Array_Random` (`self.ViableLocations`)))
  (bind _returnvalue (`KismetMathLibrary.InRange_FloatFloat` (`self.Shift Time Left`) 115.0 125.0))
  (bind (_value _returnvalue_2) (`BlueprintMapLibrary.Map_Find` (`self.Locations&Rotations`) _outitem))
  (bind _output_get (set `self.Player Character` `Player Character`))
  (set `self.Shift Time Left` (`/Game/FirstPerson/Blueprints/BP_FirstPersonCharacter.ShiftTimeLeft` `Player Character`))
  (`KismetSystemLibrary.Delay` 1.0)
  (bind _keys (`BlueprintMapLibrary.Map_Keys` (`self.Locations&Rotations`)))
  (for _array_element _keys
    (bind _returnvalue_x (`KismetMathLibrary.BreakVector` (`KismetMathLibrary.InverseTransformLocation` (`self.GetTransform` _output_get) _array_element)))
    (if (< _returnvalue_x 0.0)
      (`KismetArrayLibrary.Array_RemoveItem` _viablelocations _array_element)
      (elif (== (`KismetArrayLibrary.Array_Find` _viablelocations _array_element) -1)
        (`KismetArrayLibrary.Array_Add` _viablelocations _array_element))))
  (if (== `Day Number` 3)
    (if _returnvalue
      (if _returnvalue_2 :!label _label
        (`/Engine/EditorBlueprintResources/StandardMacros.DoOnce` false :!label _label_2
          (:`Completed`
            (`self.K2_TeleportTo` _outitem _value)
            (`SkeletalMeshComponent.SetAnimation` _mesh "/Game/LiminalMarket/Created_assets/sheep/Male_Standing_Pose_Anim.Male_Standing_Pose_Anim")
            (`PrimitiveComponent.SetMaterial` _mesh 0 "/Game/LiminalMarket/Created_assets/sheep/sheepbodymyuv_DefaultMaterial_BaseColor_Mat1.sheepbodymyuv_DefaultMaterial_BaseColor_Mat1")
            (set `self.CanTeleport` true)))))
    (elif (or _returnvalue (`KismetMathLibrary.InRange_FloatFloat` (`self.Shift Time Left`) 355.0 365.0))
      (goto _label))))

(event `Reset`
  (goto _label_2 :!via `Reset`))

(event `self.ReceiveTick`
  (params (DeltaSeconds :type "Float (single-precision)"))
  (bind _mesh (`self.Mesh`))
  (bind _original_location (`self.Original Location`))
  (`/Engine/EditorBlueprintResources/StandardMacros.Gate` true :!label _label_3
    (:`Exit`
      (if (and (< (`KismetMathLibrary.Vector_Distance` (`self.K2_GetActorLocation`) (`self.K2_GetActorLocation` (`GameplayStatics.GetPlayerCharacter` 0))) 150.0) (`self.CanTeleport`))
        (`/Engine/EditorBlueprintResources/StandardMacros.DoOnce` false :!label _label_4
          (:`Completed`
            (`self.OnTooClose`)
            (`self.K2_TeleportTo` _original_location (`BlueprintMapLibrary.Map_Find` (`self.Locations&Rotations`) _original_location))
            (`SkeletalMeshComponent.SetAnimation` _mesh "/Game/LiminalMarket/Created_assets/sheep/Female_Standing_Pose_3__Anim.Female_Standing_Pose_3__Anim")
            (`PrimitiveComponent.SetMaterial` _mesh 0 "/Game/LiminalMarket/Created_assets/sheep/sheepbodymyuv_DefaultMaterial_BaseColor_Mat.sheepbodymyuv_DefaultMaterial_BaseColor_Mat")
            (set `self.CanTeleport` false)
            (`self.Reset`)))))))

(event `self.ReceiveActorBeginOverlap`
  (params (OtherActor :type "Actor Object Reference"))
  (if (== OtherActor (`GameplayStatics.GetPlayerCharacter` 0))
    (goto _label_3 :!via `Open`)))

(event `ResetEvent`
  (goto _label_4 :!via `Reset`))

(event `self.ReceiveActorEndOverlap`
  (params (OtherActor :type "Actor Object Reference"))
  (if (== OtherActor (`GameplayStatics.GetPlayerCharacter` 0))
    (goto _label_3 :!via `Close`)))

(event `OnTooClose`
  (bind _player_character (`self.Player Character`))
  (bind _player_character_2 (`self.Player Character`))
  (bind _output_get (set `self.Old Location` (`self.K2_GetActorLocation` _player_character_2)))
  (bind (_x _y _z) (`KismetMathLibrary.BreakVector3f` _output_get))
  (`self.K2_TeleportTo` _player_character_2 (`KismetMathLibrary.MakeVector` _x _y (- _z 1475.0)) (`self.K2_GetActorRotation` _player_character_2))
  (`self.NoSounds`)
  (`KismetSystemLibrary.Delay` 15.0)
  (`self.K2_TeleportTo` _player_character (`self.Old Location`) (`self.K2_GetActorRotation` _player_character))
  (`self.SoundsPlease`)
  (`self.ResetEvent`))

(event `NoSounds`
  (`GameplayStatics.SetSoundMixClassOverride` "/Game/Sounds/MasterMix.MasterMix" "/Engine/EngineSounds/Master.Master" 0.0 1.0 0.5)
  (`GameplayStatics.PushSoundMixModifier` "/Game/Sounds/MasterMix.MasterMix"))

(event `SoundsPlease`
  (`GameplayStatics.SetSoundMixClassOverride` "/Game/Sounds/MasterMix.MasterMix" "/Engine/EngineSounds/Master.Master" (`/Game/Blueprints/Widgets/HUDMain.MasterVolume` (`/Game/FirstPerson/Blueprints/BP_FirstPersonCharacter.HUDRef` (`self.Player Character`))) 1.0 0.5)
  (`GameplayStatics.PushSoundMixModifier` "/Game/Sounds/MasterMix.MasterMix"))

(fn `UserConstructionScript`)