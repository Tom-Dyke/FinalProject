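; BP_NPC_Baker is the baker NPC, whose dialogue changes as the game's days pass.
; On BeginPlay it casts the player character to BP_FirstPersonCharacter and binds to its NewDay event.
; Days one to three each assign that day's dialogue tree to the DialogueComponent.
; On day four it sets the player's BakerVanish flag and destroys itself, removing the baker from the world.
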(event `self.ReceiveBeginPlay`
  (bind _asbp_first_person_character (cast `/Game/FirstPerson/Blueprints/BP_FirstPersonCharacter` (`GameplayStatics.GetPlayerCharacter` 0)))
  (bind _output_get (set `self.As BP First Person Character` _asbp_first_person_character))
  (add `/Game/FirstPerson/Blueprints/BP_FirstPersonCharacter.NewDay` _output_get (delegate `NextDay`)))

(event `NextDay`
  (params (`Day Number` :type Integer))
  (switch `int` `Day Number`
    (:`1`
      (set `/Game/Blueprints/Components/DialogueComponent.Dialogue Tree` (`self.Dialogue Tree Day 1`) (`self.DialogueComponent`)))
    (:`2`
      (set `/Game/Blueprints/Components/DialogueComponent.Dialogue Tree` (`self.Dialogue Tree Day 2`) (`self.DialogueComponent`)))
    (:`3`
      (set `/Game/Blueprints/Components/DialogueComponent.Dialogue Tree` (`self.Dialogue Tree Day 3`) (`self.DialogueComponent`)))
    (:`4`
      (set `/Game/FirstPerson/Blueprints/BP_FirstPersonCharacter.BakerVanish` true (`self.As BP First Person Character`))
      (`self.K2_DestroyActor`))))

(fn `UserConstructionScript`)