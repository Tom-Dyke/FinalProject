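; BP_Customer is an AI shopper with a randomized male or female look that adds to the player's score.
; BeginPlay spawns its AI controller, runs the behavior tree and seeds the blackboard with shop locations, player reference and waiting flags.
; StartTimer drives WaitTime through a timeline, then sends the customer to EndVector to be destroyed.
; Calculate awards a point per found item, scaled down once the wait passes a threshold.
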(event `StartTimer`
  (bind (_direction _waittime) (`Timeline|Timeline` :!via `PlayFromStart`)
    (:`Update`
      (set `self.Wait Time` _waittime))
    (:`Finished`
      (`|AIMoveTo` null (`self.End Vector`) null
        (:`OnSuccess`
          (`self.K2_DestroyActor`))))))

(event `self.ReceiveDestroyed`
  (bind _customer_ai (`self.Customer AI`))
  (`/Engine/EditorBlueprintResources/StandardMacros.IsValid` _customer_ai
    (:`Is Valid`
      (`BrainComponent.StopLogic` (`AIController.BrainComponent` _customer_ai) "leave"))))

(event `self.ReceiveBeginPlay`
  (`self.ChooseBody`)
  (bind _returnvalue (`|SpawnActorFromClass` "/Game/Blueprints/AI/Customer/CustomerAIController.CustomerAIController_C" (`self.GetTransform`) "Undefined" "OverrideRootScale" null null))
  (set `self.Customer AI` _returnvalue)
  (`AIController.RunBehaviorTree` (`self.Customer AI`) "/Game/Blueprints/AI/Customer/CustomerTree.CustomerTree")
  (bind _blackboardcomponent (`AIController.UseBlackboard` (`self.Customer AI`) "/Game/Blueprints/AI/Customer/CustomerBlackboard.CustomerBlackboard"))
  (`BlackboardComponent.SetValueAsObject` _blackboardcomponent "CustomerPawn" self)
  (`BlackboardComponent.SetValueAsVector` _blackboardcomponent "CheckoutLocation" (`self.Checkout`))
  (`BlackboardComponent.SetValueAsVector` _blackboardcomponent "BakeryLocation" (`self.Bakery`))
  (`BlackboardComponent.SetValueAsVector` _blackboardcomponent "PharmacyLocation" (`self.Pharmacy`))
  (`BlackboardComponent.SetValueAsVector` _blackboardcomponent "FishmongerLocation" (`self.Fishmonger`))
  (bind _asbp_first_person_character (cast `/Game/FirstPerson/Blueprints/BP_FirstPersonCharacter` (`GameplayStatics.GetPlayerCharacter` 0)))
  (set `self.As BP First Person Character` _asbp_first_person_character)
  (`BlackboardComponent.SetValueAsBool` _blackboardcomponent "CustomerWaiting" (`/Game/FirstPerson/Blueprints/BP_FirstPersonCharacter.CustomerWaiting` _asbp_first_person_character))
  (`BlackboardComponent.SetValueAsBool` _blackboardcomponent "CustomerWaitingBakery" (`/Game/FirstPerson/Blueprints/BP_FirstPersonCharacter.CustomerWaitingBakery` _asbp_first_person_character))
  (`BlackboardComponent.SetValueAsObject` _blackboardcomponent "Player Character" _asbp_first_person_character))

(event `ChooseBody`
  (bind _mesh (`self.Mesh`))
  (switch `int` (`KismetMathLibrary.RandomIntegerInRange` 0 1)
    (:`0`
      (`SkeletalMeshComponent.SetSkeletalMeshAsset` (`self.Mesh`) "/Game/LiminalMarket/models/Walking_With_Shopping_Bag.Walking_With_Shopping_Bag")
      (`PrimitiveComponent.SetMaterial` (`self.Mesh`) 0 (`KismetArrayLibrary.Array_Random` (`self.Male`))))
    (:`1`
      (`SkeletalMeshComponent.SetSkeletalMeshAsset` _mesh "/Game/LiminalMarket/models/Walking_With_Shopping_Bagfemale.Walking_With_Shopping_Bagfemale")
      (`SceneComponent.SetWorldScale3D` _mesh (`KismetMathLibrary.Conv_DoubleToVector` 0.5))
      (`PrimitiveComponent.SetMaterial` (`self.Mesh`) 0 (`KismetArrayLibrary.Array_Random` (`self.Female`))))))

(event `No Item`
  (params (`Shelf To Check` :type "/Game/Blueprints/Components/ShelfBlueprint Object Reference")))

(event `Calculate`
  (bind _as_bp_first_person_character (`self.As BP First Person Character`))
  (bind _playerscore (`/Game/FirstPerson/Blueprints/BP_FirstPersonCharacter.PlayerScore` _as_bp_first_person_character))
  (if (< (- (`self.Wait Time`) 60.0) 0.0)
    (bind _output_get (set `self.Points` (`KismetMathLibrary.Conv_IntToDouble` (`KismetArrayLibrary.Array_Length` (`self.FoundItems`)))))
    (set `/Game/FirstPerson/Blueprints/BP_FirstPersonCharacter.PlayerScore` (+ _output_get _playerscore) _as_bp_first_person_character)
    (else
      (bind _output_get_2 (set `self.Points` (* (/ (- 180.0 (`self.Wait Time`)) 180.0) (`KismetArrayLibrary.Array_Length` (`self.FoundItems`)))))
      (set `/Game/FirstPerson/Blueprints/BP_FirstPersonCharacter.PlayerScore` (+ _playerscore _output_get_2) _as_bp_first_person_character))))

(fn `UserConstructionScript`)