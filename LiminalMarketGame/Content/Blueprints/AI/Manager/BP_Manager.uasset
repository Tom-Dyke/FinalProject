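; BP_Manager is the AI manager actor, which starts its behavior tree when play begins.
; BeginPlay spawns a manager AI controller at its own transform, runs the tree on it and applies the manager blackboard, with no Possess call in this graph.
; It seeds the blackboard with the first-person player character, itself as the manager pawn, and a one-time copy of the player's clocked-in state.
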(event `self.ReceiveBeginPlay`
  (bind _asbp_first_person_character (cast `/Game/FirstPerson/Blueprints/BP_FirstPersonCharacter` (`GameplayStatics.GetPlayerCharacter` 0) :!pure true))
  (bind _returnvalue (`|SpawnActorFromClass` "/Game/Blueprints/AI/Manager/ManagerAIController.ManagerAIController_C" (`self.GetTransform`) "Undefined" "OverrideRootScale" null null))
  (set `self.ManagerAIController` _returnvalue)
  (`AIController.RunBehaviorTree` (`self.ManagerAIController`) "/Game/Blueprints/AI/Manager/ManagerTree.ManagerTree")
  (bind _blackboardcomponent (`AIController.UseBlackboard` (`self.ManagerAIController`) "/Game/Blueprints/AI/Manager/MangerBlackboard.MangerBlackboard"))
  (`BlackboardComponent.SetValueAsObject` _blackboardcomponent "PlayerCharacter" _asbp_first_person_character)
  (`BlackboardComponent.SetValueAsBool` _blackboardcomponent "Clocked-In" (`/Game/FirstPerson/Blueprints/BP_FirstPersonCharacter.ClockedIn` _asbp_first_person_character))
  (`BlackboardComponent.SetValueAsObject` _blackboardcomponent "ManagerPawn" self))

(fn `UserConstructionScript`)